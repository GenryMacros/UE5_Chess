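; PieceSphere is a hoverable sphere that displays a chess piece: bishop, knight, rook or queen.
; ML_SetPiece stores the type, reveals the matching mesh and uses SetTexture to give it a black or white dynamic material instance.
; Cursor events drive two timelines that ease the sphere's Color parameter from its current value toward the select or basic color.
; A flag stops the hover timeline once the cursor leaves.
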(event `self.Sphere.OnBeginCursorOver`
  (params (TouchedComponent :type "PrimitiveComponent Object Reference"))
  (set `self.stop_over_animation` false)
  (bind (_direction _alpha) (`Timeline|Timeline` :!via `PlayFromStart` :!label _label)
    (:`Update`
      (if (`self.stop_over_animation`)
        (goto _label :!via `Stop`)
        (else
          (bind _output_get (set `self.current_color` (`KismetMathLibrary.VLerp` (`self.current_color`) (`self.select_sphere_color`) _alpha)))
          (`MeshComponent.SetVectorParameterValueOnMaterials` (`self.Sphere`) "Color" _output_get))))))

(event `self.Sphere.OnEndCursorOver`
  (params (TouchedComponent :type "PrimitiveComponent Object Reference"))
  (set `self.stop_over_animation` true)
  (bind (_direction _alpha) (`Timeline|Timeline_1` :!via `PlayFromStart`)
    (:`Update`
      (bind _output_get (set `self.current_color` (`KismetMathLibrary.VLerp` (`self.current_color`) (`self.basic_sphere_color`) _alpha)))
      (`MeshComponent.SetVectorParameterValueOnMaterials` (`self.Sphere`) "Color" _output_get))))

(event `ML_SetPiece`
  (params (piece_type :type "/Game/Blueprints/PieceNames Enum" :default "NewEnumerator0") (is_black :type Boolean))
  (bind _knight (`self.Knight`))
  (bind _queen (`self.Queen`))
  (bind _bishop (`self.Bishop`))
  (bind _rook (`self.Rook`))
  (bind _output_get (set `self.repr_piece` piece_type))
  (switch `/Game/Blueprints/PieceNames` _output_get
    (:`NewEnumerator1`
      (`SceneComponent.SetVisibility` _bishop true false)
      (`self.Set texture` _bishop is_black))
    (:`NewEnumerator2`
      (`SceneComponent.SetVisibility` _knight true false)
      (`self.Set texture` _knight is_black))
    (:`NewEnumerator3`
      (`SceneComponent.SetVisibility` _rook true false)
      (`self.Set texture` _rook is_black))
    (:`NewEnumerator4`
      (`SceneComponent.SetVisibility` _queen true false)
      (`self.Set texture` _queen is_black))))

(fn `Set texture`
  (params (mesh :type "StaticMeshComponent Object Reference") (is_black :type Boolean))
  (if is_black
    (`PrimitiveComponent.CreateDynamicMaterialInstance` mesh 0 "/Game/Materials/Piece_Materials/Black_Instance.Black_Instance" "None")
    (else
      (`PrimitiveComponent.CreateDynamicMaterialInstance` mesh 0 "/Game/Materials/Piece_Materials/White_Instance.White_Instance" "None"))))

(fn `UserConstructionScript`)