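; Board actor that spawns 3D text labels along the left and bottom edges of a tile-map grid.
; GenerateNames places a Text3DActor per name, spaced by the TileMap's IndexMultiplier, and stores them in LeftAssets and BottomAssets.
; ClearTextArray destroys earlier labels before respawning.
; The bottom pass is nested in the left loop, so it rebuilds every iteration, and it counts by LeftNames' length.
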(fn `clearTextArray`
  (params (NewParam :type "Array of Text3DActor Object Reference"))
  (for _array_element NewParam
    (`/Engine/EditorBlueprintResources/StandardMacros.IsValid` _array_element
      (:`Is Valid`
        (`self.K2_DestroyActor` _array_element))))
  (`KismetArrayLibrary.Array_Clear` NewParam))

(fn `generateNames`
  (bind _index_multiplier (`/Game/Blueprints/TileMap.index_multiplier` (`self.tile_map`)))
  (bind _index_multiplier_2 (`/Game/Blueprints/TileMap.index_multiplier` (`self.tile_map`)))
  (`self.clearTextArray` (`self.left_assets`))
  (for _index (range (+ (`KismetArrayLibrary.Array_Length` (`self.left_names`)) 1))
    (bind _result (`/Engine/EditorBlueprintResources/StandardMacros.NegateFloat` (* _index_multiplier_2 0.8))
      (:`  `
        (bind _returnvalue (`|SpawnActorFromClass` "/Script/Text3D.Text3DActor" (`KismetMathLibrary.MakeTransform` (`KismetMathLibrary.MakeVector` (- (* _index_multiplier_2 _index) (* _index_multiplier_2 0.1)) _result 7.0) (struct :`Pitch` -90.0)) "Undefined" "OverrideRootScale" null null))
        (`Text3DComponent.SetText` (`Text3DActor.Text3DComponent` _returnvalue) (`KismetTextLibrary.Conv_StringToText` (`|GetArrayItem` (`self.left_names`) _index)))
        (`KismetArrayLibrary.Array_Add` (`self.left_assets`) _returnvalue)
        (`self.clearTextArray` (`self.bottom_assets`))
        (for _index_2 (range (+ (`KismetArrayLibrary.Array_Length` (`self.left_names`)) 1))
          (bind _result_2 (`/Engine/EditorBlueprintResources/StandardMacros.NegateFloat` (* _index_multiplier 0.85))
            (:`  `
              (bind _returnvalue_2 (`|SpawnActorFromClass` "/Script/Text3D.Text3DActor" (`KismetMathLibrary.MakeTransform` (`KismetMathLibrary.MakeVector` _result_2 (- (* _index_multiplier _index_2) (* _index_multiplier 0.13)) 7.0) (struct :`Pitch` -90.0)) "Undefined" "OverrideRootScale" null null))
              (`Text3DComponent.SetText` (`Text3DActor.Text3DComponent` _returnvalue_2) (`KismetTextLibrary.Conv_StringToText` (`|GetArrayItem` (`self.bottom_names`) _index_2)))
              (`KismetArrayLibrary.Array_Add` (`self.bottom_assets`) _returnvalue_2))))))))

(fn `UserConstructionScript`)