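; ObservePawn is an observer camera pawn with a visible mouse cursor and mouse-over events.
; BeginPlay adds the observer Enhanced Input mapping context to the first player controller.
; Right mouse press and release toggle a look mode that gates mouse-driven pitch and yaw input.
; The mouse wheel zooms by stepping the spring arm length, with a minimum limit on zooming in but none on zooming out.
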(event `self.ReceiveBeginPlay`
  (bind _returnvalue (`GameplayStatics.GetPlayerController` 0))
  (bind _returnvalue_2 (pcsubsystem `EnhancedInputLocalPlayerSubsystem` _returnvalue))
  (set `PlayerController.bShowMouseCursor` true _returnvalue)
  (`/Engine/EditorBlueprintResources/StandardMacros.IsValid` _returnvalue_2
    (:`Is Valid`
      (`EnhancedInputSubsystemInterface.AddMappingContext` _returnvalue_2 "/Game/Controls/ObserverMappingContext.ObserverMappingContext" 0 (struct))
      (set `PlayerController.bEnableMouseOverEvents` true (`GameplayStatics.GetPlayerController` 0)))))

(event `EnhancedInput|/Game/Controls/Actions/IA_Mouse_Up_Down`
  (params (ActionValue :type "Float (double-precision)") (ElapsedSeconds :type "Float (double-precision)") (TriggeredSeconds :type "Float (double-precision)") (InputAction :type "InputAction Object Reference" :default "/Game/Controls/Actions/IA_Mouse_Up_Down.IA_Mouse_Up_Down"))
  (:`Triggered`
    (if (`self.is_mouse_move_mode`)
      (`self.AddControllerPitchInput` ActionValue))))

(event `EnhancedInput|/Game/Controls/Actions/IA_Mouse_Right_Left`
  (params (ActionValue :type "Float (double-precision)") (ElapsedSeconds :type "Float (double-precision)") (TriggeredSeconds :type "Float (double-precision)") (InputAction :type "InputAction Object Reference" :default "/Game/Controls/Actions/IA_Mouse_Right_Left.IA_Mouse_Right_Left"))
  (:`Triggered`
    (if (`self.is_mouse_move_mode`)
      (`self.AddControllerYawInput` ActionValue))))

(event `EnhancedInput|/Game/Controls/Actions/IA_RMB_CLICK`
  (params (ActionValue :type "Float (double-precision)") (ElapsedSeconds :type "Float (double-precision)") (TriggeredSeconds :type "Float (double-precision)") (InputAction :type "InputAction Object Reference" :default "/Game/Controls/Actions/IA_RMB_CLICK.IA_RMB_CLICK"))
  (:`Triggered`
    (set `self.is_mouse_move_mode` true)))

(event `EnhancedInput|/Game/Controls/Actions/IA_RMB_RELEASED`
  (params (ActionValue :type "Float (double-precision)") (ElapsedSeconds :type "Float (double-precision)") (TriggeredSeconds :type "Float (double-precision)") (InputAction :type "InputAction Object Reference" :default "/Game/Controls/Actions/IA_RMB_RELEASED.IA_RMB_RELEASED"))
  (:`Triggered`
    (set `self.is_mouse_move_mode` false)))

(event `EnhancedInput|/Game/Controls/Actions/IA_Mouse_Wheel_Up`
  (params (ActionValue :type "Float (double-precision)") (ElapsedSeconds :type "Float (double-precision)") (TriggeredSeconds :type "Float (double-precision)") (InputAction :type "InputAction Object Reference" :default "/Game/Controls/Actions/IA_Mouse_Wheel_Up.IA_Mouse_Wheel_Up"))
  (bind _springarm (`self.SpringArm`))
  (bind _targetarmlength (`SpringArmComponent.TargetArmLength` _springarm))
  (:`Triggered`
    (if (> _targetarmlength 600.0)
      (set `SpringArmComponent.TargetArmLength` (+ _targetarmlength -60.0) _springarm))))

(event `EnhancedInput|/Game/Controls/Actions/IA_Mouse_Wheel_Down`
  (params (ActionValue :type "Float (double-precision)") (ElapsedSeconds :type "Float (double-precision)") (TriggeredSeconds :type "Float (double-precision)") (InputAction :type "InputAction Object Reference" :default "/Game/Controls/Actions/IA_Mouse_Wheel_Down.IA_Mouse_Wheel_Down"))
  (bind _springarm (`self.SpringArm`))
  (:`Triggered`
    (set `SpringArmComponent.TargetArmLength` (+ (`SpringArmComponent.TargetArmLength` _springarm) 60.0) _springarm)))

(fn `UserConstructionScript`)