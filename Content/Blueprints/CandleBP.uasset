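; Candle actor Blueprint that makes its point light flicker once play begins.
; BeginPlay starts the Flickering timeline, which sets the light intensity on every update.
; Each update lerps between randomized bounds just below MinIntensity and just above MaxIntensity, using the timeline's alpha plus a small random offset for irregular jitter.
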(event `self.ReceiveBeginPlay`
  (bind _min_intensity (`self.min_intensity`))
  (bind _max_intensity (`self.max_intensity`))
  (bind (_direction _flickering_alpha) (`Timeline|Flickering`)
    (:`Update`
      (`LightComponent.SetIntensity` (`self.PointLight`) (`KismetMathLibrary.Lerp` (`KismetMathLibrary.RandomFloatInRange` (- _min_intensity 100.0) _min_intensity) (`KismetMathLibrary.RandomFloatInRange` _max_intensity (+ _max_intensity 100.0)) (+ _flickering_alpha (`KismetMathLibrary.RandomFloatInRange` 0.1 0.3)))))))

(fn `UserConstructionScript`)