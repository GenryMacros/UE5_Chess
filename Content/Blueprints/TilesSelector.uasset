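; Chess tile selection helper that tracks and highlights the tiles a picked piece can move to.
; SelectPiece clears the previous selection, then marks tiles returned by the piece if its color matches the current turn.
; FilterSelected simulates each move by swapping tiles, tests opponent attacks with the game mode's IsCheckmate, then restores the board.
; As wired, it drops failing moves only when the target tile holds a piece.
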(event `self.ReceiveBeginPlay`
  (bind _aschess_player_controller (cast `/Game/Blueprints/Global/ChessPlayerController` (`GameplayStatics.GetPlayerController` 0)))
  (set `self.player_controller` _aschess_player_controller)
  (bind _aschess_game_state (cast `/Game/Blueprints/Global/ChessGameState` (`GameplayStatics.GetGameState`)))
  (set `self.game_state` _aschess_game_state))

(fn `DeselectSelected`
  (for _array_element (`self.selected_tiles`)
    (`/Game/Blueprints/Tile.Deselect` _array_element)
    (`/Game/Blueprints/Tile.UnMarkAsPreMove` _array_element))
  (`KismetArrayLibrary.Array_Clear` (`self.selected_tiles`)))

(fn `FilterSelected`
  (params (Piece :type "/Game/Blueprints/Pieces/Piece Object Reference"))
  (locals (piece_original_tile :type "/Game/Blueprints/Tile Object Reference") (remembered_piece :type "/Game/Blueprints/Pieces/Piece Object Reference") (remembered_piece_info :type "/Game/Blueprints/Structs/PieceInfo Structure") (tile_map_cop :type "/Game/Blueprints/TileMap Object Reference"))
  (bind _remembered_piece (`local.remembered_piece`))
  (set `local.tile_map_cop` (`/Game/Blueprints/Global/ChessGameState.tile_map` (`self.game_state`)))
  (bind _output_get (set `local.piece_original_tile` (`/Game/Blueprints/Pieces/Piece.tile` Piece)))
  (for _array_element (`self.selected_tiles`)
    (if (!= _array_element _output_get)
      (bind _holded_piece (`/Game/Blueprints/Tile.holded_piece` _array_element))
      (`/Engine/EditorBlueprintResources/StandardMacros.IsValid` _holded_piece
        (:`Is Valid`
          (set `local.remembered_piece` _holded_piece))
        (:`Is Not Valid`
          (set `local.remembered_piece` null)))
      (set `local.remembered_piece_info` (`/Game/Blueprints/Tile.holded_piece_info` _array_element))
      (`/Game/Blueprints/TileMap.SwapTiles` (`local.tile_map_cop`) (`local.piece_original_tile`) _array_element)
      (bind _aschess_game_state (cast `/Game/Blueprints/Global/ChessGameState` (`GameplayStatics.GetGameState`)))
      (bind _tiles_under_attack (`/Game/Blueprints/Global/ChessGameState.GetAllAttackedTiles` _aschess_game_state (not (`/Game/Blueprints/Pieces/Piece.is_black` Piece))))
      (bind _aschess_game_mode (cast `/Game/Blueprints/Global/ChessGameMode` (`GameplayStatics.GetGameMode`)))
      (bind _is_checkmate (`/Game/Blueprints/Global/ChessGameMode.IsCheckmate` _aschess_game_mode _tiles_under_attack))
      (`/Game/Blueprints/TileMap.SwapTiles` (`local.tile_map_cop`) _array_element (`local.piece_original_tile`))
      (set `/Game/Blueprints/Tile.holded_piece` _remembered_piece _array_element)
      (set `/Game/Blueprints/Tile.holded_piece_info` (`local.remembered_piece_info`) _array_element)
      (`/Engine/EditorBlueprintResources/StandardMacros.IsValid` _remembered_piece
        (:`Is Valid`
          (set `/Game/Blueprints/Pieces/Piece.tile` _array_element _remembered_piece)
          (if _is_checkmate
            (`/Game/Blueprints/Tile.Deselect` _array_element)
            (`KismetArrayLibrary.Array_RemoveItem` (`self.selected_tiles`) _array_element)))))))

(fn `IsTileSelected`
  (params (tile :type "/Game/Blueprints/Tile Object Reference"))
  (returns (is_selected :type Boolean))
  (return (!= -1 (`KismetArrayLibrary.Array_Find` (`self.selected_tiles`) tile))))

(fn `SelectPiece`
  (params (Piece :type "/Game/Blueprints/Pieces/Piece Object Reference") (is_black_turn :type Boolean))
  (returns (selected :type "Array of /Game/Blueprints/Tile Object Reference"))
  (`self.DeselectSelected`)
  (if (== is_black_turn (`/Game/Blueprints/Pieces/Piece.is_black` Piece))
    (bind _aschess_game_state (cast `/Game/Blueprints/Global/ChessGameState` (`GameplayStatics.GetGameState`)))
    (bind _selected_tiles (`/Game/Blueprints/Pieces/Piece.select` Piece (`/Game/Blueprints/Global/ChessGameState.tile_map` _aschess_game_state)))
    (for _array_element _selected_tiles
      (`/Game/Blueprints/Tile.MakeSelected` _array_element)
      (`KismetArrayLibrary.Array_Add` (`self.selected_tiles`) _array_element))
    (return (`self.selected_tiles`))))

(fn `UserConstructionScript`)