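; TileMap is the chess board manager that spawns a checkered grid of Tile actors and stores them in a flat array.
; It handles tile selection, threat clearing, coordinate conversion and a signed material score, positive for white.
; SwapTiles moves a piece one way, unlinking any piece on the destination.
; Despite their names, Import2Json writes to a hardcoded JSON test file and ExportFromJson reads piece info back from it.
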(event `self.ReceiveBeginPlay`)

(event `ML_Make Non Threat All`
  (params (is_black :type Boolean))
  (for _array_element (`self.Tiles`)
    (bind (_holded_piece_info_piece_name _holded_piece_info_is_black) (break `/Game/Blueprints/Structs/PieceInfo` (`/Game/Blueprints/Tile.holded_piece_info` _array_element)))
    (if (== _holded_piece_info_is_black is_black)
      (`/Game/Blueprints/Tile.MakeNonThreat` _array_element))))

(fn `CalculateScore`
  (returns (res :type Integer))
  (locals (score :type Integer) (mod :type Integer))
  (bind _score (`local.score`))
  (bind _mod (`local.mod`))
  (for _array_element (`self.Tiles`)
    (bind (_holded_piece_info_piece_name _holded_piece_info_is_black) (break `/Game/Blueprints/Structs/PieceInfo` (`/Game/Blueprints/Tile.holded_piece_info` _array_element)))
    (if _holded_piece_info_is_black
      (set `local.mod` -1)
      (else
        (set `local.mod` 1)))
    (switch `/Game/Blueprints/PieceNames` _holded_piece_info_piece_name
      (:`NewEnumerator0`
        (set `local.score` (+ _score (* 1 _mod))))
      (:`NewEnumerator1`
        (set `local.score` (+ _score (* 3 _mod))))
      (:`NewEnumerator2`
        (set `local.score` (+ _score (* 3 _mod))))
      (:`NewEnumerator3`
        (set `local.score` (+ _score (* 5 _mod))))
      (:`NewEnumerator4`
        (set `local.score` (+ _score (* 9 _mod))))))
  (return (`local.score`)))

(fn `Clear`
  (bind _tiles (`self.Tiles`))
  (for _array_element _tiles
    (`/Engine/EditorBlueprintResources/StandardMacros.IsValid` _array_element
      (:`Is Valid`
        (`self.K2_DestroyActor` _array_element))))
  (`KismetArrayLibrary.Array_Clear` _tiles))

(fn `Coord2Index`
  (params (x :type Integer) (y :type Integer))
  (returns (index :type Integer))
  (if (or (< x 0) (< y 0) (>= x (`self.tile_width`)) (>= y (`self.tile_height`)))
    (return -1)
    (else
      (return (+ (* (`self.tile_width`) x) y)))))

(fn `DeselectAll`
  (for _array_element (`self.Tiles`)
    (`self.DeselectTile` _array_element)))

(fn `DeselectTile`
  (params (tile :type "/Game/Blueprints/Tile Object Reference"))
  (`/Game/Blueprints/Tile.Deselect` tile))

(fn `ExportFromJson`
  (bind _outjsonobject (`JsonBlueprintFunctionLibrary.FromFile` (make `FilePath` "C:\\Project Dream\\Unreal\\Truly_Chess\\test.json")))
  (for (_array_element _array_index) (`self.Tiles`)
    (bind (_outvalue _returnvalue) (`|GetJsonField` _outjsonobject (`KismetStringLibrary.Conv_IntToString` _array_index)))
    (if _returnvalue
      (bind _outvalue_2 (`|GetJsonField` _outvalue "piece_name"))
      (bind _outvalue_3 (`|GetJsonField` _outvalue "is_black"))
      (set `/Game/Blueprints/Tile.holded_piece_info` (make `/Game/Blueprints/Structs/PieceInfo` (cast `/Game/Blueprints/PieceNames` _outvalue_2) _outvalue_3) _array_element)
      (else
        (set `/Game/Blueprints/Tile.holded_piece_info` (make `/Game/Blueprints/Structs/PieceInfo` "NewEnumerator6") _array_element)))))

(fn `Import2Json`
  (bind _jsonobjectwrapper (make `JsonObjectWrapper`))
  (bind _jsonobjectwrapper_2 (make `JsonObjectWrapper`))
  (for (_array_element _array_index) (`self.Tiles`)
    (bind (_holded_piece_info_piece_name _holded_piece_info_is_black) (break `/Game/Blueprints/Structs/PieceInfo` (`/Game/Blueprints/Tile.holded_piece_info` _array_element)))
    (`|SetJsonField` _jsonobjectwrapper "piece_name" (`KismetMathLibrary.Conv_ByteToInt` _holded_piece_info_piece_name))
    (`|SetJsonField` _jsonobjectwrapper "is_black" _holded_piece_info_is_black)
    (`|SetJsonField` _jsonobjectwrapper_2 (`KismetStringLibrary.Conv_IntToString` _array_index) _jsonobjectwrapper))
  (`JsonBlueprintFunctionLibrary.ToFile` _jsonobjectwrapper_2 (make `FilePath` "C:\\Project Dream\\Unreal\\Truly_Chess\\test.json")))

(fn `Index2Coord`
  (params (i :type Integer) (j :type Integer))
  (returns (coord :type "Vector Structure"))
  (bind _index_multiplier (`self.index_multiplier`))
  (return (`KismetMathLibrary.MakeVector` (* i _index_multiplier) (* j _index_multiplier))))

(fn `Index2String`
  (params (i :type Integer) (j :type Integer))
  (returns (strigified :type String) (ReturnValue :type "/Game/Blueprints/BottomMark Enum")))

(fn `Make Non Threat All`
  (for _array_element (`self.Tiles`)
    (`/Game/Blueprints/Tile.MakeNonThreat` _array_element)))

(fn `Reset map`
  (bind _index_multiplier (`self.index_multiplier`))
  (`self.Clear`)
  (for _index (range (`self.tile_width`))
    (for _index_2 (range (`self.tile_height`))
      (bind _returnvalue (`|SpawnActorFromClass` "/Game/Blueprints/Tile.Tile_C" (`KismetMathLibrary.MakeTransform` (`KismetMathLibrary.MakeVector` (* _index _index_multiplier) (* _index_2 _index_multiplier))) "Undefined" "OverrideRootScale" null (make `/Game/Blueprints/Structs/Coord` _index _index_2) null))
      (if (`KismetMathLibrary.Conv_IntToBool` (mod (+ _index_2 _index) 2))
        (`PrimitiveComponent.CreateDynamicMaterialInstance` (`/Game/Blueprints/Tile.base` _returnvalue) 0 (`self.white_material`) "None")
        (else
          (`PrimitiveComponent.CreateDynamicMaterialInstance` (`/Game/Blueprints/Tile.base` _returnvalue) 0 (`self.black_material`) "None")))
      (bind _returnvalue_2 (`PrimitiveComponent.CreateDynamicMaterialInstance` (`/Game/Blueprints/Tile.select` _returnvalue) 0 null "None"))
      (`MaterialInstanceDynamic.SetScalarParameterValue` _returnvalue_2 "Opacity" 0.0)
      (set `/Game/Blueprints/Tile.holded_piece_info` (make `/Game/Blueprints/Structs/PieceInfo` "NewEnumerator6") _returnvalue)
      (`KismetArrayLibrary.Array_Add` (`self.Tiles`) _returnvalue))))

(fn `SelectTile`
  (params (tile :type "/Game/Blueprints/Tile Object Reference"))
  (`/Game/Blueprints/Tile.MakeSelected` tile))

(fn `SwapTiles`
  (params (tile1 :type "/Game/Blueprints/Tile Object Reference") (tile2 :type "/Game/Blueprints/Tile Object Reference"))
  (locals (tile1_holded_piece :type "/Game/Blueprints/Pieces/Piece Object Reference"))
  (bind _tile1_holded_piece (`local.tile1_holded_piece`))
  (bind _holded_piece (`/Game/Blueprints/Tile.holded_piece` tile1))
  (bind _holded_piece_2 (`/Game/Blueprints/Tile.holded_piece` tile2))
  (bind (_holded_piece_info_piece_name _holded_piece_info_is_black) (break `/Game/Blueprints/Structs/PieceInfo` (`/Game/Blueprints/Tile.holded_piece_info` tile1)))
  (if (!= tile1 tile2)
    (`/Engine/EditorBlueprintResources/StandardMacros.IsValid` _holded_piece
      (:`Is Valid`
        (set `local.tile1_holded_piece` _holded_piece)
        (set `/Game/Blueprints/Tile.holded_piece_info` (make `/Game/Blueprints/Structs/PieceInfo` _holded_piece_info_piece_name _holded_piece_info_is_black) tile2)
        (set `/Game/Blueprints/Tile.holded_piece_info` (make `/Game/Blueprints/Structs/PieceInfo` "NewEnumerator6") tile1)
        (`/Engine/EditorBlueprintResources/StandardMacros.IsValid` _holded_piece_2
          (:`Is Valid`
            (set `/Game/Blueprints/Pieces/Piece.tile` null _holded_piece_2))
          (:`Is Not Valid`
            _))
        (set `/Game/Blueprints/Tile.holded_piece` _tile1_holded_piece tile2)
        (set `/Game/Blueprints/Pieces/Piece.tile` tile2 _tile1_holded_piece)
        (set `/Game/Blueprints/Tile.holded_piece` null tile1)))))

(fn `UserConstructionScript`)