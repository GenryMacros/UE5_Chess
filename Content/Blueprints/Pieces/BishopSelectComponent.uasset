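; Piece component for a bishop in a chess-style tile game, providing a ray-style tile selection along a given direction.
; SelectOnAxis steps from the start tile by the X/Y direction, converting coordinates to TileMap indices for up to roughly the map's width.
; It adds empty tiles (piece enum 6), stops at the first occupied tile, including it only for an opposite color, or at an invalid index.
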(fn `selectOnAxis`
  (params (selected_tiles :type "Array of /Game/Blueprints/Tile Object Reference") (tile_map :type "/Game/Blueprints/TileMap Object Reference") (x_dir :type Integer) (y_dir :type Integer) (start_tile :type "/Game/Blueprints/Tile Object Reference"))
  (locals (current_x :type Integer) (current_y :type Integer))
  (bind _tiles (`/Game/Blueprints/TileMap.Tiles` tile_map))
  (bind (_coords_x _coords_y) (break `/Game/Blueprints/Structs/Coord` (`/Game/Blueprints/Tile.coords` start_tile)))
  (bind (_holded_piece_info_piece_name _holded_piece_info_is_black) (break `/Game/Blueprints/Structs/PieceInfo` (`/Game/Blueprints/Tile.holded_piece_info` start_tile)))
  (set `local.current_x` (+ _coords_x x_dir))
  (set `local.current_y` (+ _coords_y y_dir))
  (for _ (range (+ (`/Game/Blueprints/TileMap.tile_width` tile_map) 1))
    (bind _index (`/Game/Blueprints/TileMap.Coord2Index` tile_map (`local.current_x`) (`local.current_y`)))
    (if (`KismetArrayLibrary.Array_IsValidIndex` _tiles _index)
      (bind _output (`|GetArrayItem` _tiles _index))
      (bind (_holded_piece_info_piece_name_2 _holded_piece_info_is_black_2) (break `/Game/Blueprints/Structs/PieceInfo` (`/Game/Blueprints/Tile.holded_piece_info` _output)))
      (if (!= (`KismetMathLibrary.Conv_ByteToInt` _holded_piece_info_piece_name_2) 6)
        (if (!= _holded_piece_info_is_black_2 _holded_piece_info_is_black)
          (`KismetArrayLibrary.Array_Add` selected_tiles _output)
          (break)
          (else
            (break)))
        (else
          (`KismetArrayLibrary.Array_Add` selected_tiles _output)
          (set `local.current_x` (+ (`local.current_x`) x_dir))
          (set `local.current_y` (+ (`local.current_y`) y_dir))))
      (else
        (break)))))