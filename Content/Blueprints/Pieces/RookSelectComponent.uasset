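; Rook piece component that finds the tiles reachable in a straight line from a start tile on the board's tile map.
; SelectOnAxis scans one direction along X or Y, adding empty tiles and stopping at the first occupied one, which it includes only if the colors differ.
; Backward scans reuse the ascending loop by iterating negated indices and taking Abs, and both axes use TileWidth as the upper bound.
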(fn `selectOnAxis`
  (params (selected_tiles :type "Array of /Game/Blueprints/Tile Object Reference") (is_right :type Boolean) (tile_map :type "/Game/Blueprints/TileMap Object Reference") (is_x :type Boolean) (start_tile :type "/Game/Blueprints/Tile Object Reference"))
  (locals (end_index :type Integer) (cur_x_coord :type Integer) (cur_y_coord :type Integer) (cur_start_index :type Integer))
  (bind _tiles (`/Game/Blueprints/TileMap.Tiles` tile_map))
  (bind _cur_start_index (`local.cur_start_index`))
  (bind (_coords_x _coords_y) (break `/Game/Blueprints/Structs/Coord` (`/Game/Blueprints/Tile.coords` start_tile)))
  (bind (_holded_piece_info_piece_name _holded_piece_info_is_black) (break `/Game/Blueprints/Structs/PieceInfo` (`/Game/Blueprints/Tile.holded_piece_info` start_tile)))
  (set `local.cur_y_coord` _coords_y)
  (set `local.cur_x_coord` _coords_x)
  (if is_x
    (set `local.cur_start_index` _coords_x)
    (else
      (set `local.cur_start_index` _coords_y)))
  (if is_right
    (set `local.end_index` (- (`/Game/Blueprints/TileMap.tile_width` tile_map) 1))
    (set `local.cur_start_index` (+ _cur_start_index 1))
    (else
      (set `local.end_index` 0)
      (set `local.cur_start_index` (* (- _cur_start_index 1) -1))))
  (for _index (range (`local.cur_start_index`) (+ (`local.end_index`) 1))
    (if is_x
      (bind _returnvalue (`KismetMathLibrary.Abs_Int` _index))
      (bind _output_get (set `local.cur_x_coord` _returnvalue))
      (else
        (bind _output_get_2 (set `local.cur_y_coord` _returnvalue))))
    (bind _index_2 (`/Game/Blueprints/TileMap.Coord2Index` tile_map _output_get _output_get_2))
    (if (`KismetArrayLibrary.Array_IsValidIndex` _tiles _index_2)
      (bind _output (`|GetArrayItem` _tiles _index_2))
      (bind (_holded_piece_info_piece_name_2 _holded_piece_info_is_black_2) (break `/Game/Blueprints/Structs/PieceInfo` (`/Game/Blueprints/Tile.holded_piece_info` _output)))
      (if (!= (`KismetMathLibrary.Conv_ByteToInt` _holded_piece_info_piece_name_2) (`KismetMathLibrary.Conv_ByteToInt` (enumliteral `/Game/Blueprints/PieceNames` "NewEnumerator6")))
        (if (!= _holded_piece_info_is_black_2 _holded_piece_info_is_black)
          (`KismetArrayLibrary.Array_Add` selected_tiles _output)
          (break)
          (else
            (break)))
        (else
          (`KismetArrayLibrary.Array_Add` selected_tiles _output)))
      (else
        (break)))))