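; Rook chess piece Blueprint that supplies its selectable tiles, material and piece-type enum.
; Select calls RookSelectComponent.SelectOnAxis once for each of the four axis directions from the current tile, then adds that tile itself to the selection.
; PostMove flags the rook as moved on its first move but always returns no follow-up move.
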(fn `GetPieceName`
  (returns (name :type "/Game/Blueprints/PieceNames Enum"))
  (return "NewEnumerator3"))

(fn `PostMove`
  (params (new_tile :type "/Game/Blueprints/Tile Object Reference") (tile_map :type "/Game/Blueprints/TileMap Object Reference"))
  (returns (is_moved :type Boolean) (piece :type "/Game/Blueprints/Pieces/Piece Object Reference") (to :type "Vector Structure"))
  (if (not (`self.is_moved`))
    (set `self.is_moved` true)
    (return false null (0.0 0.0 0.0))
    (else
      (return false null (0.0 0.0 0.0)))))

(fn `select`
  (params (tile_map :type "/Game/Blueprints/TileMap Object Reference"))
  (returns (selected_tiles :type "Array of /Game/Blueprints/Tile Object Reference"))
  (locals (current_selected :type "Array of /Game/Blueprints/Tile Object Reference"))
  (bind _current_selected (`local.current_selected`))
  (bind _current_selected_2 (`local.current_selected`))
  (bind _tile (`self.tile`))
  (bind _rookselectcomponent (`self.RookSelectComponent`))
  (`/Engine/EditorBlueprintResources/StandardMacros.IsValid` (`self.tile`)
    (:`Is Valid`
      (`/Game/Blueprints/Pieces/RookSelectComponent.selectOnAxis` _rookselectcomponent _current_selected_2 false tile_map true _tile)
      (`/Game/Blueprints/Pieces/RookSelectComponent.selectOnAxis` _rookselectcomponent _current_selected_2 true tile_map true _tile)
      (`/Game/Blueprints/Pieces/RookSelectComponent.selectOnAxis` _rookselectcomponent _current_selected_2 false tile_map false _tile)
      (`/Game/Blueprints/Pieces/RookSelectComponent.selectOnAxis` _rookselectcomponent _current_selected_2 true tile_map false _tile)
      (`KismetArrayLibrary.Array_Add` _current_selected (`self.tile`)))
    (:`Is Not Valid`
      _))
  (return _current_selected))

(fn `Set Material`
  (params (material :type "MaterialInterface Object Reference"))
  (`PrimitiveComponent.SetMaterial` (`self.piece_0`) 0 material))

(fn `UserConstructionScript`
  (`parent.UserConstructionScript`))