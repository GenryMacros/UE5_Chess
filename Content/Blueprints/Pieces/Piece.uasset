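; Base actor for a board game piece on a tile map, with mostly stub functions that appear intended for child pieces to override.
; CorrectLocation shifts the actor by a fixed offset, ignoring its IsBlack input, and GetTile returns the stored tile.
; Select and SetMaterial are empty, PostMove reports no move, and GetPieceName returns a default enum value.
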(fn `CorrectLocation`
  (params (is_black :type Boolean))
  (returns (piece :type "/Game/Blueprints/Pieces/Piece Object Reference"))
  (`self.K2_SetActorLocation` (+ (`KismetMathLibrary.MakeVector` -44.0 -52.0 36.0) (`self.K2_GetActorLocation`)))
  (return self))

(fn `GetPieceName`
  (returns (name :type "/Game/Blueprints/PieceNames Enum"))
  (return "NewEnumerator0"))

(fn `GetTile`
  (returns (tile :type "/Game/Blueprints/Tile Object Reference"))
  (return (`self.tile`)))

(fn `PostMove`
  (params (new_tile :type "/Game/Blueprints/Tile Object Reference") (tile_map :type "/Game/Blueprints/TileMap Object Reference"))
  (returns (is_moved :type Boolean) (piece :type "/Game/Blueprints/Pieces/Piece Object Reference") (to :type "Vector Structure"))
  (return false null (0.0 0.0 0.0)))

(fn `select`
  (params (tile_map :type "/Game/Blueprints/TileMap Object Reference"))
  (returns (selected_tiles :type "Array of /Game/Blueprints/Tile Object Reference"))
  (return))

(fn `Set Material`
  (params (material :type "MaterialInterface Object Reference")))

(fn `UserConstructionScript`)