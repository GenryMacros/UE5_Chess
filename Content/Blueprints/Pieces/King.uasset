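; King chess piece Blueprint that supplies its selectable tiles and handles castling.
; Select gathers its own and adjacent empty or opposing tiles, using a world-distance check to discard wrapped indices, then CastlingSelect adds two-square castle targets.
; Castling requires no IsInCheckmate flag, a clear path and an unmoved same-colour Rook.
; PostMove marks the King moved and, on castling, reassigns the Rook's tile data, returning that piece and its destination.
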(fn `CastlingSelect`
  (params (`Tile map` :type "/Game/Blueprints/TileMap Object Reference") (current_selected :type "Array of /Game/Blueprints/Tile Object Reference"))
  (bind _tiles (`/Game/Blueprints/TileMap.Tiles` `Tile map`))
  (bind (_coords_x _coords_y) (break `/Game/Blueprints/Structs/Coord` (`/Game/Blueprints/Tile.coords` (`self.tile`))))
  (if (and (not (`self.is_in_checkmate`)) (not (`self.is_moved`)))
    (bind _index (`/Game/Blueprints/TileMap.Coord2Index` `Tile map` _coords_x (+ _coords_y 3)))
    (bind _index_2 (`/Game/Blueprints/TileMap.Coord2Index` `Tile map` _coords_x (- _coords_y 4)))
    (bind _is_castling_possible (`self.IsCastlingPossible` (`|GetArrayItem` _tiles _index) `Tile map`))
    (if _is_castling_possible
      (bind _index_3 (`/Game/Blueprints/TileMap.Coord2Index` `Tile map` _coords_x (+ _coords_y 2)))
      (`KismetArrayLibrary.Array_Add` current_selected (`|GetArrayItem` (`/Game/Blueprints/TileMap.Tiles` `Tile map`) _index_3)))
    (bind _is_castling_possible_2 (`self.IsCastlingPossible` (`|GetArrayItem` _tiles _index_2) `Tile map`))
    (if _is_castling_possible_2
      (bind _index_4 (`/Game/Blueprints/TileMap.Coord2Index` `Tile map` _coords_x (- _coords_y 2)))
      (`KismetArrayLibrary.Array_Add` current_selected (`|GetArrayItem` (`/Game/Blueprints/TileMap.Tiles` `Tile map`) _index_4)))))

(fn `GetPieceName`
  (returns (name :type "/Game/Blueprints/PieceNames Enum"))
  (return "NewEnumerator5"))

(fn `IsCastlingPossible`
  (params (rook_tile :type "/Game/Blueprints/Tile Object Reference") (tile_map :type "/Game/Blueprints/TileMap Object Reference"))
  (returns (is_castling_possible :type Boolean))
  (locals (is_piece_in_a_way :type Boolean))
  (bind (_coords_x _coords_y) (break `/Game/Blueprints/Structs/Coord` (`/Game/Blueprints/Tile.coords` rook_tile)))
  (bind _holded_piece (`/Game/Blueprints/Tile.holded_piece` rook_tile))
  (bind (_coords_x_2 _coords_y_2) (break `/Game/Blueprints/Structs/Coord` (`/Game/Blueprints/Tile.coords` (`self.tile`))))
  (bind _returnvalue (- _coords_y _coords_y_2))
  (bind _returnvalue_2 (/ (`KismetMathLibrary.Abs_Int` _returnvalue) _returnvalue))
  (bind _returnvalue_3 (+ _coords_y_2 _returnvalue_2))
  (`/Engine/EditorBlueprintResources/StandardMacros.IsValid` rook_tile
    (:`Is Valid`
      (if (`self.is_moved`)
        (return false)
        (else
          (for _index (range (+ (`KismetMathLibrary.Min` _returnvalue_3 _coords_y) (`KismetMathLibrary.Abs_Int` (`KismetMathLibrary.Min` _returnvalue_2))) (`KismetMathLibrary.Max` _returnvalue_3 _coords_y))
            (bind _index_2 (`/Game/Blueprints/TileMap.Coord2Index` tile_map _coords_x_2 _index))
            (bind _holded_piece_info_piece_name (break `/Game/Blueprints/Structs/PieceInfo` (`/Game/Blueprints/Tile.holded_piece_info` (`|GetArrayItem` (`/Game/Blueprints/TileMap.Tiles` tile_map) _index_2))))
            (if (!= (`KismetMathLibrary.Conv_ByteToInt` (enumliteral `/Game/Blueprints/PieceNames` "NewEnumerator6")) (`KismetMathLibrary.Conv_ByteToInt` _holded_piece_info_piece_name))
              (set `local.is_piece_in_a_way` true)
              (break)))
          (if (not (`local.is_piece_in_a_way`))
            (`/Engine/EditorBlueprintResources/StandardMacros.IsValid` _holded_piece
              (:`Is Valid`
                (bind _asrook (cast `/Game/Blueprints/Pieces/Rook` _holded_piece)
                  (:`then`
                    (return (and (== (`self.is_black`) (`/Game/Blueprints/Pieces/Piece.is_black` _asrook)) (not (`/Game/Blueprints/Pieces/Rook.is_moved` _asrook)))))
                  (:`CastFailed`
                    _)))))
          (return false))))
    (:`Is Not Valid`
      (return false))))

(fn `PostMove`
  (params (new_tile :type "/Game/Blueprints/Tile Object Reference") (tile_map :type "/Game/Blueprints/TileMap Object Reference"))
  (returns (is_moved :type Boolean) (piece :type "/Game/Blueprints/Pieces/Piece Object Reference") (to :type "Vector Structure"))
  (locals (rook_tile :type "/Game/Blueprints/Tile Object Reference"))
  (bind _rook_tile (`local.rook_tile`))
  (bind _tiles (`/Game/Blueprints/TileMap.Tiles` tile_map))
  (bind (_coords_x _coords_y) (break `/Game/Blueprints/Structs/Coord` (`/Game/Blueprints/Tile.coords` new_tile)))
  (bind _holded_piece (`/Game/Blueprints/Tile.holded_piece` _rook_tile))
  (bind (_coords_x_2 _coords_y_2) (break `/Game/Blueprints/Structs/Coord` (`/Game/Blueprints/Tile.coords` (`self.tile`))))
  (bind _returnvalue (- _coords_y _coords_y_2))
  (bind _returnvalue_2 (`KismetMathLibrary.Abs_Int` _returnvalue))
  (bind _returnvalue_3 (/ _returnvalue_2 _returnvalue))
  (bind _returnvalue_4 (+ _returnvalue_3 _coords_y))
  (if (not (`self.is_moved`))
    (if (> _returnvalue_2 1)
      (bind _index (`/Game/Blueprints/TileMap.Coord2Index` tile_map _coords_x_2 _returnvalue_4))
      (bind _output (`|GetArrayItem` _tiles _index))
      (`/Engine/EditorBlueprintResources/StandardMacros.IsValid` (`/Game/Blueprints/Tile.holded_piece` _output)
        (:`Is Valid`
          (set `local.rook_tile` _output))
        (:`Is Not Valid`
          (bind _index_2 (`/Game/Blueprints/TileMap.Coord2Index` tile_map _coords_x_2 (- _returnvalue_4 1)))
          (set `local.rook_tile` (`|GetArrayItem` _tiles _index_2))))
      (bind _index_3 (`/Game/Blueprints/TileMap.Coord2Index` tile_map _coords_x_2 (+ _coords_y_2 _returnvalue_3)))
      (bind _output_2 (`|GetArrayItem` _tiles _index_3))
      (bind _output_get (set `/Game/Blueprints/Tile.holded_piece` _holded_piece _output_2))
      (set `/Game/Blueprints/Tile.holded_piece_info` (`/Game/Blueprints/Tile.holded_piece_info` _rook_tile) _output_2)
      (set `/Game/Blueprints/Pieces/Piece.tile` _output_2 _holded_piece)
      (set `/Game/Blueprints/Tile.holded_piece` null _rook_tile)
      (set `/Game/Blueprints/Tile.holded_piece_info` (struct) _rook_tile)
      (set `self.is_moved` true)
      (return true _output_get (+ (`self.K2_GetActorLocation` _output_2) (-44.0 -52.0 36.0)))
      (else
        (set `self.is_moved` true))))
  (return false null (0.0 0.0 0.0)))

(fn `select`
  (params (tile_map :type "/Game/Blueprints/TileMap Object Reference"))
  (returns (selected_tiles :type "Array of /Game/Blueprints/Tile Object Reference"))
  (locals (current_selected :type "Array of /Game/Blueprints/Tile Object Reference"))
  (bind _tiles (`/Game/Blueprints/TileMap.Tiles` tile_map))
  (bind _tile (`self.tile`))
  (bind (_returnvalue_x _returnvalue_y) (`KismetMathLibrary.BreakVector` (`self.K2_GetActorLocation` _tile)))
  (bind (_coords_x _coords_y) (break `/Game/Blueprints/Structs/Coord` (`/Game/Blueprints/Tile.coords` (`self.tile`))))
  (`/Engine/EditorBlueprintResources/StandardMacros.IsValid` (`self.tile`)
    (:`Is Valid`
      (for _index (range (- _coords_x 1) (+ (+ _coords_x 1) 1))
        (for _index_2 (range (- _coords_y 1) (+ (+ _coords_y 1) 1))
          (bind _index_3 (`/Game/Blueprints/TileMap.Coord2Index` tile_map _index _index_2))
          (if (`KismetArrayLibrary.Array_IsValidIndex` _tiles _index_3)
            (bind _output (`|GetArrayItem` _tiles _index_3))
            (bind (_returnvalue_x_2 _returnvalue_y_2) (`KismetMathLibrary.BreakVector` (`self.K2_GetActorLocation` _output)))
            (bind (_holded_piece_info_piece_name _holded_piece_info_is_black) (break `/Game/Blueprints/Structs/PieceInfo` (`/Game/Blueprints/Tile.holded_piece_info` _output)))
            (if (and (and (<= (`KismetMathLibrary.Abs` (- _returnvalue_x_2 _returnvalue_x)) 145.0) (<= (`KismetMathLibrary.Abs` (- _returnvalue_y_2 _returnvalue_y)) 145.0)) (or (!= (`self.is_black`) _holded_piece_info_is_black) (== (`KismetMathLibrary.Conv_ByteToInt` _holded_piece_info_piece_name) (`KismetMathLibrary.Conv_ByteToInt` (enumliteral `/Game/Blueprints/PieceNames` "NewEnumerator6"))) (== _output _tile)))
              (`KismetArrayLibrary.Array_Add` (`local.current_selected`) _output))))))
    (:`Is Not Valid`
      _))
  (`self.CastlingSelect` tile_map (`local.current_selected`))
  (return (`local.current_selected`)))

(fn `Set Material`
  (params (material :type "MaterialInterface Object Reference"))
  (`PrimitiveComponent.SetMaterial` (`self.piece_0`) 0 material))

(fn `UserConstructionScript`
  (`parent.UserConstructionScript`))