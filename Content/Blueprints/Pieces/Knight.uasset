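; Knight chess piece Blueprint that finds the tiles it can move to and supplies its piece type.
; Select adds each DirsToCheck offset to the current tile's coordinates, converts it to a tile map index and keeps valid tiles matching a color or piece-name test, plus its own tile.
; CorrectLocation offsets and turns the actor according to color, and SetMaterial applies a material to the mesh.
; BeginPlay, overlap and Tick events are disabled stubs.
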(fn `CorrectLocation`
  (params (is_black :type Boolean))
  (returns (piece :type "/Game/Blueprints/Pieces/Piece Object Reference"))
  (bind _returnvalue (`self.GetActorScale3D`))
  (if is_black
    (`self.K2_SetActorTransform` (`KismetMathLibrary.MakeTransform` (+ (`KismetMathLibrary.MakeVector` 52.0 -44.0 36.0) (`self.K2_GetActorLocation`)) (struct :`Yaw` 90.0) _returnvalue))
    (else
      (`self.K2_SetActorTransform` (`KismetMathLibrary.MakeTransform` (+ (`KismetMathLibrary.MakeVector` -52.0 45.0 36.0) (`self.K2_GetActorLocation`)) (struct :`Yaw` -90.0) _returnvalue))))
  (return self))

(fn `GetPieceName`
  (returns (name :type "/Game/Blueprints/PieceNames Enum"))
  (return "NewEnumerator2"))

(fn `select`
  (params (tile_map :type "/Game/Blueprints/TileMap Object Reference"))
  (returns (selected_tiles :type "Array of /Game/Blueprints/Tile Object Reference"))
  (locals (dirs_to_check :type "Array of /Game/Blueprints/Structs/Coord Structure") (current_selected :type "Array of /Game/Blueprints/Tile Object Reference"))
  (bind _tiles (`/Game/Blueprints/TileMap.Tiles` tile_map))
  (bind _current_selected (`local.current_selected`))
  (bind (_coords_x _coords_y) (break `/Game/Blueprints/Structs/Coord` (`/Game/Blueprints/Tile.coords` (`self.tile`))))
  (`/Engine/EditorBlueprintResources/StandardMacros.IsValid` (`self.tile`)
    (:`Is Valid`
      (for _array_element (`local.dirs_to_check`)
        (bind _index (`/Game/Blueprints/TileMap.Coord2Index` tile_map (+ (break `/Game/Blueprints/Structs/Coord` _array_element) _coords_x) (+ (`.y_9_5BD02C3F48B234B61681E3A6610D6505` (break `/Game/Blueprints/Structs/Coord` _array_element)) _coords_y)))
        (if (`KismetArrayLibrary.Array_IsValidIndex` _tiles _index)
          (if true
            (bind _output (`|GetArrayItem` _tiles _index))
            (bind (_holded_piece_info_piece_name _holded_piece_info_is_black) (break `/Game/Blueprints/Structs/PieceInfo` (`/Game/Blueprints/Tile.holded_piece_info` _output)))
            (if (or (!= (`self.is_black`) _holded_piece_info_is_black) (== (`KismetMathLibrary.Conv_ByteToInt` (enumliteral `/Game/Blueprints/PieceNames` "NewEnumerator6")) (`KismetMathLibrary.Conv_ByteToInt` _holded_piece_info_piece_name)) (== (`self.tile`) _output))
              (`KismetArrayLibrary.Array_Add` (`local.current_selected`) _output)))))
      (`KismetArrayLibrary.Array_Add` _current_selected (`self.tile`))
      (return _current_selected))))

(fn `Set Material`
  (params (material :type "MaterialInterface Object Reference"))
  (`PrimitiveComponent.SetMaterial` (`self.piece_0`) 0 material))

(fn `UserConstructionScript`
  (`parent.UserConstructionScript`))