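; Chess pawn piece Blueprint that supplies its selectable tiles, piece type and post-move result.
; Select gathers its own tile, empty tiles one step ahead (two from InitialX) and diagonal enemy captures, with direction set by color.
; Captures also pass a world-distance check against the pawn's tile.
; PostMove returns true when the pawn's Tile is on row 6 for white or row 1 for black, with a zero vector.
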(fn `GetPieceName`
  (returns (name :type "/Game/Blueprints/PieceNames Enum"))
  (return "NewEnumerator0"))

(fn `PostMove`
  (params (new_tile :type "/Game/Blueprints/Tile Object Reference") (tile_map :type "/Game/Blueprints/TileMap Object Reference"))
  (returns (is_moved :type Boolean) (piece :type "/Game/Blueprints/Pieces/Piece Object Reference") (to :type "Vector Structure"))
  (bind _coords_x (break `/Game/Blueprints/Structs/Coord` (`/Game/Blueprints/Tile.coords` (`self.tile`))))
  (if (or (and (== _coords_x 6) (not (`self.is_black`))) (and (== _coords_x 1) (`self.is_black`)))
    (return true null (0.0 0.0 0.0))
    (else
      (return false null (0.0 0.0 0.0)))))

(fn `select`
  (params (tile_map :type "/Game/Blueprints/TileMap Object Reference"))
  (returns (selected_tiles :type "Array of /Game/Blueprints/Tile Object Reference"))
  (locals (last_checking_x :type Integer) (current_selected :type "Array of /Game/Blueprints/Tile Object Reference") (move_dir :type Integer) (ys_to_check :type "Array of Integer"))
  (bind _tiles (`/Game/Blueprints/TileMap.Tiles` tile_map))
  (bind _ys_to_check (`local.ys_to_check`))
  (bind _last_checking_x (`local.last_checking_x`))
  (bind _move_dir (`local.move_dir`))
  (bind _tile (`self.tile`))
  (bind _tiles_2 (`/Game/Blueprints/TileMap.Tiles` tile_map))
  (bind (_returnvalue_x _returnvalue_y) (`KismetMathLibrary.BreakVector` (`self.K2_GetActorLocation` (`self.tile`))))
  (bind (_coords_x _coords_y) (break `/Game/Blueprints/Structs/Coord` (`/Game/Blueprints/Tile.coords` (`self.tile`))))
  (bind (_coords_x_2 _coords_y_2) (break `/Game/Blueprints/Structs/Coord` (`/Game/Blueprints/Tile.coords` (`self.tile`))))
  (bind _returnvalue (+ _coords_x (`local.move_dir`)))
  (`/Engine/EditorBlueprintResources/StandardMacros.IsValid` _tile
    (:`Is Valid`
      (`KismetArrayLibrary.Array_Add` (`local.current_selected`) _tile)
      (if (`self.is_black`)
        (set `local.move_dir` -1)
        (else
          (set `local.move_dir` 1)))
      (if (== _coords_x (`self.initial_x`))
        (set `local.last_checking_x` (+ _coords_x (* 2 _move_dir)))
        (else
          (set `local.last_checking_x` (+ _coords_x _move_dir))))
      (for _index (range (`KismetMathLibrary.Min` _returnvalue _last_checking_x) (+ (`KismetMathLibrary.Max` _returnvalue _last_checking_x) 1))
        (bind _index_2 (`/Game/Blueprints/TileMap.Coord2Index` tile_map _index _coords_y))
        (if (`KismetArrayLibrary.Array_IsValidIndex` _tiles _index_2)
          (bind _output (`|GetArrayItem` _tiles _index_2))
          (bind _res (`/Game/Blueprints/Tile.IsWithoutPiece` _output))
          (if _res
            (`KismetArrayLibrary.Array_Add` (`local.current_selected`) _output)
            (else
              (if (not (`self.is_black`)) :!label _label
                (break))))
          (else
            (goto _label))))
      (`KismetArrayLibrary.Array_Add` _ys_to_check (+ 1 _coords_y_2))
      (`KismetArrayLibrary.Array_Add` _ys_to_check (+ _coords_y_2 -1))
      (for _array_element _ys_to_check
        (bind _index_3 (`/Game/Blueprints/TileMap.Coord2Index` tile_map (+ _coords_x_2 (`local.move_dir`)) _array_element))
        (if (`KismetArrayLibrary.Array_IsValidIndex` _tiles_2 _index_3)
          (bind _output_2 (`|GetArrayItem` _tiles_2 _index_3))
          (bind _res_2 (`/Game/Blueprints/Tile.IsWithoutPiece` _output_2))
          (bind (_holded_piece_info_piece_name _holded_piece_info_is_black) (break `/Game/Blueprints/Structs/PieceInfo` (`/Game/Blueprints/Tile.holded_piece_info` _output_2)))
          (bind (_returnvalue_x_2 _returnvalue_y_2) (`KismetMathLibrary.BreakVector` (`self.K2_GetActorLocation` _output_2)))
          (if (and (!= (`self.is_black`) _holded_piece_info_is_black) (not _res_2) (<= (`KismetMathLibrary.Abs` (- _returnvalue_y _returnvalue_y_2)) 145.0) (<= (`KismetMathLibrary.Abs` (- _returnvalue_x _returnvalue_x_2)) 145.0))
            (`KismetArrayLibrary.Array_Add` (`local.current_selected`) _output_2))))
      (return (`local.current_selected`)))
    (:`Is Not Valid`
      (return))))

(fn `Set Material`
  (params (material :type "MaterialInterface Object Reference"))
  (`PrimitiveComponent.SetMaterial` (`self.piece_0`) 0 material))

(fn `UserConstructionScript`
  (`parent.UserConstructionScript`))