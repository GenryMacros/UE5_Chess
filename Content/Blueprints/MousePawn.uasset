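; Player pawn for a chess game that drives the orbit camera and mouse interaction with pieces and in-game buttons.
; Right-drag rotates the view and the wheel zooms the spring arm; left-click traces from the cursor to grab own pieces, pick promotion pieces or press buttons.
; Tick drags the grabbed piece via the ChessPlayerController and traces down to pre-mark the target tile.
; On release, a spawned TilesSelector checks that tile before the controller makes the move.
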(event `self.ReceiveBeginPlay`
  (bind _player_controller (`self.player_controller`))
  (bind _returnvalue (pcsubsystem `EnhancedInputLocalPlayerSubsystem` _player_controller))
  (bind _aschess_player_controller (cast `/Game/Blueprints/Global/ChessPlayerController` (`GameplayStatics.GetPlayerController` 0)))
  (set `self.player_controller` _aschess_player_controller)
  (set `PlayerController.bShowMouseCursor` true _player_controller)
  (`/Engine/EditorBlueprintResources/StandardMacros.IsValid` _returnvalue
    (:`Is Valid`
      (`EnhancedInputSubsystemInterface.AddMappingContext` _returnvalue "/Game/Controls/ChessMappingContext.ChessMappingContext" -1 (struct))
      (bind _returnvalue_2 (`|SpawnActorFromClass` "/Game/Blueprints/TilesSelector.TilesSelector_C" (`KismetMathLibrary.MakeTransform` (0.0 0.0 0.0)) "Undefined" "OverrideRootScale" null null))
      (set `self.tile_selector` _returnvalue_2))))

(event `EnhancedInput|/Game/Controls/Actions/IA_Mouse_Up_Down`
  (params (ActionValue :type "Float (double-precision)") (ElapsedSeconds :type "Float (double-precision)") (TriggeredSeconds :type "Float (double-precision)") (InputAction :type "InputAction Object Reference" :default "/Game/Controls/Actions/IA_Mouse_Up_Down.IA_Mouse_Up_Down"))
  (:`Triggered`
    (if (`self.is_mouse_move_mode`)
      (`self.AddControllerPitchInput` ActionValue))))

(event `EnhancedInput|/Game/Controls/Actions/IA_Mouse_Right_Left`
  (params (ActionValue :type "Float (double-precision)") (ElapsedSeconds :type "Float (double-precision)") (TriggeredSeconds :type "Float (double-precision)") (InputAction :type "InputAction Object Reference" :default "/Game/Controls/Actions/IA_Mouse_Right_Left.IA_Mouse_Right_Left"))
  (:`Triggered`
    (if (`self.is_mouse_move_mode`)
      (`self.AddControllerYawInput` ActionValue))))

(event `EnhancedInput|/Game/Controls/Actions/IA_Mouse_Wheel_Up`
  (params (ActionValue :type "Float (double-precision)") (ElapsedSeconds :type "Float (double-precision)") (TriggeredSeconds :type "Float (double-precision)") (InputAction :type "InputAction Object Reference" :default "/Game/Controls/Actions/IA_Mouse_Wheel_Up.IA_Mouse_Wheel_Up"))
  (bind _springarm (`self.SpringArm`))
  (bind _targetarmlength (`SpringArmComponent.TargetArmLength` _springarm))
  (:`Triggered`
    (if (> _targetarmlength 600.0)
      (set `SpringArmComponent.TargetArmLength` (+ _targetarmlength -60.0) _springarm))))

(event `EnhancedInput|/Game/Controls/Actions/IA_Mouse_Wheel_Down`
  (params (ActionValue :type "Float (double-precision)") (ElapsedSeconds :type "Float (double-precision)") (TriggeredSeconds :type "Float (double-precision)") (InputAction :type "InputAction Object Reference" :default "/Game/Controls/Actions/IA_Mouse_Wheel_Down.IA_Mouse_Wheel_Down"))
  (bind _springarm (`self.SpringArm`))
  (:`Triggered`
    (set `SpringArmComponent.TargetArmLength` (+ (`SpringArmComponent.TargetArmLength` _springarm) 60.0) _springarm)))

(event `EnhancedInput|/Game/Controls/Actions/IA_RMB_CLICK`
  (params (ActionValue :type "Float (double-precision)") (ElapsedSeconds :type "Float (double-precision)") (TriggeredSeconds :type "Float (double-precision)") (InputAction :type "InputAction Object Reference" :default "/Game/Controls/Actions/IA_RMB_CLICK.IA_RMB_CLICK"))
  (:`Triggered`
    (set `self.is_mouse_move_mode` true)))

(event `EnhancedInput|/Game/Controls/Actions/IA_RMB_RELEASED`
  (params (ActionValue :type "Float (double-precision)") (ElapsedSeconds :type "Float (double-precision)") (TriggeredSeconds :type "Float (double-precision)") (InputAction :type "InputAction Object Reference" :default "/Game/Controls/Actions/IA_RMB_RELEASED.IA_RMB_RELEASED"))
  (:`Triggered`
    (set `self.is_mouse_move_mode` false)))

(event `EnhancedInput|/Game/Controls/Actions/IA_LMB_CLICK`
  (params (ActionValue :type "Float (double-precision)") (ElapsedSeconds :type "Float (double-precision)") (TriggeredSeconds :type "Float (double-precision)") (InputAction :type "InputAction Object Reference" :default "/Game/Controls/Actions/IA_LMB_CLICK.IA_LMB_CLICK"))
  (bind (_worldlocation _worlddirection _returnvalue) (`PlayerController.DeprojectMousePositionToWorld` (`self.player_controller`)))
  (:`Triggered`
    (if (`/Game/Blueprints/Global/ChessPlayerController.Is In Restart` (`self.player_controller`))
      (bind _actor (`self.GetTraceHitActor` :!label _label))
      (bind _asin_game_button (cast `/Game/Blueprints/UI/InGameButton` _actor))
      (`/Game/Blueprints/UI/InGameButton.onClick` _asin_game_button)
      (else
        (bind _is_gg (`/Game/Blueprints/Global/ChessPlayerController.IsGGState` (`self.player_controller`)))
        (if _is_gg
          (goto _label)
          (else
            (bind _is_my_turn (`/Game/Blueprints/Global/ChessPlayerController.IsMyTurn` (`self.player_controller`)))
            (if _is_my_turn
              (if (`/Game/Blueprints/Global/ChessPlayerController.is_pawn_transform_mode` (`self.player_controller`))
                (bind _actor_2 (`self.GetTraceHitActor`))
                (bind _aspiece_sphere (cast `/Game/Blueprints/PieceSphere` _actor_2)
                  (:`then`
                    (`/Game/Blueprints/Global/ChessPlayerController.SV_FinalizePawnTransformation` (`self.player_controller`) _aspiece_sphere))
                  (:`CastFailed`
                    (bind _asin_game_button_2 (cast `/Game/Blueprints/UI/InGameButton` _actor_2))
                    (`/Game/Blueprints/UI/InGameButton.onClick` _asin_game_button_2)))
                (elif _returnvalue
                  (bind (_outhit _returnvalue_2) (`KismetSystemLibrary.LineTraceSingle` _worldlocation (+ _worldlocation (* _worlddirection 10000.0)) "TraceTypeQuery1"))
                  (if _returnvalue_2
                    (if (== (`SceneComponent.Mobility` (`.HitComponent` (`GameplayStatics.BreakHitResult` _outhit))) (`KismetMathLibrary.Conv_ByteToInt` (enumliteral `EComponentMobility` "Movable")))
                      (bind (_bblockinghit _binitialoverlap _time _distance _location _impactpoint _normal _impactnormal _physmat _hitactor) (`GameplayStatics.BreakHitResult` _outhit))
                      (set `self.originalDistanceToObject` (`KismetMathLibrary.Conv_DoubleToVector` _distance))
                      (bind _aspiece (cast `/Game/Blueprints/Pieces/Piece` _hitactor)
                        (:`then`
                          (if (== (`/Game/Blueprints/Pieces/Piece.is_black` _aspiece) (`/Game/Blueprints/Global/ChessPlayerController.is_black` (`self.player_controller`)))
                            (set `self.grabbedPiece` _aspiece)
                            (set `self.relativeGrabLocation` (`KismetMathLibrary.InverseTransformLocation` (`KismetMathLibrary.Conv_VectorToTransform` (`self.K2_GetActorLocation` _aspiece)) _location))
                            (`/Game/Blueprints/TilesSelector.SelectPiece` (`self.tile_selector`) _aspiece (`/Game/Blueprints/Global/ChessPlayerController.is_black` (`self.player_controller`)))))
                        (:`CastFailed`
                          (bind _asin_game_button_3 (cast `/Game/Blueprints/UI/InGameButton` _hitactor))
                          (`/Game/Blueprints/UI/InGameButton.onClick` _asin_game_button_3))))))))))))))

(event `EnhancedInput|/Game/Controls/Actions/IA_LMB_RELEASED`
  (params (ActionValue :type "Float (double-precision)") (ElapsedSeconds :type "Float (double-precision)") (TriggeredSeconds :type "Float (double-precision)") (InputAction :type "InputAction Object Reference" :default "/Game/Controls/Actions/IA_LMB_RELEASED.IA_LMB_RELEASED"))
  (bind _grabbedpiece (`self.grabbedPiece`))
  (bind _current2go (`self.current2Go`))
  (:`Triggered`
    (`/Engine/EditorBlueprintResources/StandardMacros.IsValid` (`self.grabbedPiece`)
      (:`Is Valid`
        (bind _is_selected (`/Game/Blueprints/TilesSelector.IsTileSelected` (`self.tile_selector`) _current2go))
        (if (not _is_selected)
          (set `self.current2Go` (`/Game/Blueprints/Pieces/Piece.tile` _grabbedpiece)))
        (`/Game/Blueprints/Global/ChessPlayerController.SV_EV_MakeMove` (`self.player_controller`) _grabbedpiece _current2go)
        (`/Game/Blueprints/TilesSelector.DeselectSelected` (`self.tile_selector`))
        (set `self.relativeGrabLocation` (0.0 0.0 0.0))
        (set `self.grabbedPiece` null)))))

(event `self.ReceiveTick`
  (params (DeltaSeconds :type "Float (single-precision)"))
  (bind _grabbedpiece (`self.grabbedPiece`))
  (bind (_worldlocation _worlddirection) (`PlayerController.DeprojectMousePositionToWorld` (`GameplayStatics.GetPlayerController` 0)))
  (`/Engine/EditorBlueprintResources/StandardMacros.IsValid` _grabbedpiece
    (:`Is Valid`
      (`self.Unmark Down Tile`)
      (`/Game/Blueprints/Global/ChessPlayerController.SV_EV_ChangeActorLocation` (`self.player_controller`) _grabbedpiece (`KismetMathLibrary.InverseTransformLocation` (`KismetMathLibrary.Conv_VectorToTransform` (`self.relativeGrabLocation`)) (+ _worldlocation (* _worlddirection (`self.originalDistanceToObject`)))))
      (`self.Mark Down Tile`))))

(fn `GetTraceHitActor`
  (returns (actor :type "Actor Object Reference"))
  (bind _player_controller (`self.player_controller`))
  (bind (_worldlocation _worlddirection) (`PlayerController.DeprojectMousePositionToWorld` _player_controller))
  (bind _outhit (`KismetSystemLibrary.LineTraceSingle` _worldlocation (+ _worldlocation (* _worlddirection 10000.0)) "TraceTypeQuery1" false (`/Game/Blueprints/Graveyard.bodies` (`/Game/Blueprints/Global/ChessGameState.graveyard` (`/Game/Blueprints/Global/ChessPlayerController.game_state` _player_controller)))))
  (return (`.HitActor` (`GameplayStatics.BreakHitResult` _outhit))))

(fn `Mark Down Tile`
  (locals (down_dir :type "Vector Structure" :default (0.0 0.0 -1.0)))
  (bind _returnvalue (`self.K2_GetActorLocation` (`self.grabbedPiece`)))
  (bind (_outhit _returnvalue_2) (`KismetSystemLibrary.LineTraceSingle` _returnvalue (+ _returnvalue (* (`local.down_dir`) 1000.0)) "TraceTypeQuery2"))
  (if _returnvalue_2
    (bind (_bblockinghit _binitialoverlap _time _distance _location _impactpoint _normal _impactnormal _physmat _hitactor) (`GameplayStatics.BreakHitResult` _outhit))
    (`/Engine/EditorBlueprintResources/StandardMacros.IsValid` _hitactor
      (:`Is Valid`
        (bind _astile (cast `/Game/Blueprints/Tile` _hitactor)
          (:`then`
            (`/Game/Blueprints/Tile.MarkAsPreMove` _astile)
            (set `self.current2Go` _astile))
          (:`CastFailed`
            (bind _aspiece (cast `/Game/Blueprints/Pieces/Piece` _hitactor))
            (bind _tile (`/Game/Blueprints/Pieces/Piece.tile` _aspiece))
            (`/Game/Blueprints/Tile.MarkAsPreMove` _tile)
            (set `self.current2Go` _tile))))
      (:`Is Not Valid`
        (set `self.current2Go` (`/Game/Blueprints/Pieces/Piece.tile` (`self.grabbedPiece`)) :!label _label)))
    (else
      (goto _label))))

(fn `Rotate Camera X`
  (params (is_clockwise :type Boolean))
  (locals (local_angle_step :type "Float (double-precision)" :default 0.1))
  (bind (_returnvalue_x _returnvalue_y _returnvalue_z) (`KismetMathLibrary.BreakVector` (`self.K2_GetActorLocation`)))
  (bind (_returnvalue_roll _returnvalue_pitch _returnvalue_yaw) (`KismetMathLibrary.BreakRotator` (`self.K2_GetActorRotation` null)))
  (bind _local_angle_step (`local.local_angle_step`))
  (bind _returnvalue (`KismetMathLibrary.DegCos` _local_angle_step))
  (bind _returnvalue_2 (`KismetMathLibrary.DegSin` _local_angle_step))
  (bind _returnvalue_3 (- _returnvalue_y 0.0))
  (bind _returnvalue_4 (- _returnvalue_z 0.0))
  (if is_clockwise
    (set `local.local_angle_step` 0.0)
    (else
      (set `local.local_angle_step` (* 0.0 -1.0))))
  (`self.K2_SetActorLocation` null (`KismetMathLibrary.MakeVector` _returnvalue_x (+ (+ (* _returnvalue_3 _returnvalue) (* _returnvalue_4 (* _returnvalue_2 -1.0))) 0.0) (+ (+ (* _returnvalue_3 _returnvalue_2) (* _returnvalue_4 _returnvalue)) 0.0)) false false)
  (`self.K2_SetActorRotation` null (`KismetMathLibrary.MakeRotator` (+ _returnvalue_roll (`local.local_angle_step`)) _returnvalue_pitch _returnvalue_yaw) false))

(fn `Rotate Camera Z`
  (params (change_dir :type "Float (double-precision)"))
  (locals (local_angle_step :type "Float (double-precision)" :default 0.1) (camera_view_dot :type "Vector Structure") (z_move_angle :type "Float (double-precision)"))
  (bind (_returnvalue_x _returnvalue_y _returnvalue_z) (`KismetMathLibrary.BreakVector` (`self.K2_GetActorLocation`)))
  (bind (_returnvalue_x_2 _returnvalue_y_2 _returnvalue_z_2) (`KismetMathLibrary.BreakVector` (`self.GetActorForwardVector`)))
  (bind (_returnvalue_x_3 _returnvalue_y_3 _returnvalue_z_3) (`KismetMathLibrary.BreakVector` (`self.K2_GetActorLocation`)))
  (bind (_returnvalue_roll _returnvalue_pitch _returnvalue_yaw) (`KismetMathLibrary.BreakRotator` (`self.K2_GetActorRotation` null)))
  (bind _local_angle_step (`local.local_angle_step`))
  (bind _returnvalue (`KismetMathLibrary.DegCos` _local_angle_step))
  (bind _returnvalue_2 (`KismetMathLibrary.DegSin` _local_angle_step))
  (bind _returnvalue_3 (- _returnvalue_x_3 0.0))
  (bind _returnvalue_4 (- _returnvalue_y_3 0.0))
  (bind _returnvalue_5 (* (/ _returnvalue_z _returnvalue_z_2) -1.0))
  (bind _returnvalue_6 (`KismetMathLibrary.MakeVector` (+ (* _returnvalue_x_2 _returnvalue_5) _returnvalue_x) (+ (* _returnvalue_y_2 _returnvalue_5) _returnvalue_y) (+ (* _returnvalue_5 _returnvalue_z_2) _returnvalue_z)))
  (set `local.local_angle_step` (* change_dir 0.0))
  (`self.K2_SetActorLocation` null (`KismetMathLibrary.MakeVector` (+ (+ (* _returnvalue_3 _returnvalue) (* _returnvalue_4 (* _returnvalue_2 -1.0))) 0.0) (+ (+ (* _returnvalue_3 _returnvalue_2) (* _returnvalue_4 _returnvalue)) 0.0) _returnvalue_z_3) false false)
  (`self.K2_SetActorRotation` null (`KismetMathLibrary.MakeRotator` _returnvalue_roll _returnvalue_pitch (+ _returnvalue_yaw (* (`local.change_dir`) (`KismetMathLibrary.DegAcos` (/ (`KismetMathLibrary.Dot_VectorVector` _returnvalue_6) (* (`KismetMathLibrary.VSize` (0.0 0.0 0.0)) (`KismetMathLibrary.VSize` _returnvalue_6))))))) false))

(fn `Unmark Down Tile`
  (locals (down_dir :type "Vector Structure" :default (0.0 0.0 -1.0)))
  (bind _current2go (`self.current2Go`))
  (`/Engine/EditorBlueprintResources/StandardMacros.IsValid` _current2go
    (:`Is Valid`
      (`/Game/Blueprints/Tile.UnMarkAsPreMove` _current2go))))

(fn `UserConstructionScript`)