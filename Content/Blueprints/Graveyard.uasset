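; Graveyard for captured chess pieces, lining up white and black victims in separate rows.
; Bury picks the next slot by piece color, offsets Knights, and has the passed Animator move and rescale the victim.
; BuryWhite and BuryBlack record each body in color and combined lists, stepping their next coordinates in opposite directions by CorpseStep.
; ClearBodies empties the lists without resetting those coordinates.
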(fn `Bury`
  (params (victim :type "/Game/Blueprints/Pieces/Piece Object Reference") (animator :type "/Game/Blueprints/PiecesMoveAnimator Object Reference"))
  (locals (destination :type "Vector Structure"))
  (bind _destination (`local.destination`))
  (bind (_holded_piece_info_piece_name _holded_piece_info_is_black) (break `/Game/Blueprints/Structs/PieceInfo` (`/Game/Blueprints/Tile.holded_piece_info` (`/Game/Blueprints/Pieces/Piece.tile` victim))))
  (if (not _holded_piece_info_is_black)
    (cast `/Game/Blueprints/Pieces/Knight` victim
      (:`then`
        (set `local.destination` (+ (`KismetMathLibrary.MakeVector` -26.0 22.5) (`self.next_white_body_coord`))))
      (:`CastFailed`
        (set `local.destination` (`self.next_white_body_coord`))))
    (`/Game/Blueprints/PiecesMoveAnimator.MoveResizePieceTo` animator victim _destination (* (`self.GetActorScale3D`) (`self.scale_factor`)))
    (`self.Bury White` victim)
    (else
      (cast `/Game/Blueprints/Pieces/Knight` victim
        (:`then`
          (set `local.destination` (+ (`KismetMathLibrary.MakeVector` 26.0 -22.0) (`self.next_black_body_coord`))))
        (:`CastFailed`
          (set `local.destination` (`self.next_black_body_coord`))))
      (`/Game/Blueprints/PiecesMoveAnimator.MoveResizePieceTo` animator victim _destination (* (`self.GetActorScale3D` victim) (`self.scale_factor`)))
      (`self.BuryBlack` victim))))

(fn `Bury White`
  (params (piece :type "/Game/Blueprints/Pieces/Piece Object Reference"))
  (`KismetArrayLibrary.Array_Add` (`self.white_bodies`) piece)
  (`KismetArrayLibrary.Array_Add` (`self.bodies`) piece)
  (set `self.next_white_body_coord` (+ (`self.next_white_body_coord`) (`self.corpse_step`))))

(fn `BuryBlack`
  (params (piece :type "/Game/Blueprints/Pieces/Piece Object Reference"))
  (`KismetArrayLibrary.Array_Add` (`self.black_bodies`) piece)
  (`KismetArrayLibrary.Array_Add` (`self.bodies`) piece)
  (set `self.next_black_body_coord` (- (`self.next_black_body_coord`) (`self.corpse_step`))))

(fn `ClearBodies`
  (`KismetArrayLibrary.Array_Clear` (`self.white_bodies`))
  (`KismetArrayLibrary.Array_Clear` (`self.black_bodies`))
  (`KismetArrayLibrary.Array_Clear` (`self.bodies`)))

(fn `UserConstructionScript`)