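; Board tile actor for a piece-based game that tracks its occupying piece and shows selection, pre-move and threat highlights.
; Highlights are material scalar changes: selection and pre-move share a dynamic instance made at BeginPlay, while the threat functions request one on each call.
; Setters cache piece name and color, with only SetHoldedPiece storing the reference.
; An invalid piece resets only that cached info, which the emptiness check reads.
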(event `self.ReceiveBeginPlay`
  (bind _returnvalue (`PrimitiveComponent.CreateDynamicMaterialInstance` (`self.select`) 0 null "None"))
  (set `self.select_dynamic_material` _returnvalue))

(fn `Deselect`
  (`MaterialInstanceDynamic.SetScalarParameterValue` (`self.select_dynamic_material`) "Opacity" 0.0))

(fn `IsPieceBelongs2Tile`
  (params (Piece :type "/Game/Blueprints/Pieces/Piece Object Reference"))
  (returns (is_belongs :type Boolean))
  (return (== (`/Game/Blueprints/Pieces/Piece.tile` Piece) self)))

(fn `IsWithoutPiece`
  (returns (res :type Boolean))
  (bind _holded_piece_info_piece_name (break `/Game/Blueprints/Structs/PieceInfo` (`self.holded_piece_info`)))
  (return (== (`KismetMathLibrary.Conv_ByteToInt` (enumliteral `/Game/Blueprints/PieceNames` "NewEnumerator6")) (`KismetMathLibrary.Conv_ByteToInt` _holded_piece_info_piece_name))))

(fn `MakeNonThreat`
  (bind _returnvalue (`PrimitiveComponent.CreateDynamicMaterialInstance` (`self.threat`) 0 null "None"))
  (`MaterialInstanceDynamic.SetScalarParameterValue` _returnvalue "Alpha" 1.0))

(fn `MakeSelected`
  (`MaterialInstanceDynamic.SetScalarParameterValue` (`self.select_dynamic_material`) "Opacity" 0.2))

(fn `MakeThreat`
  (bind _returnvalue (`PrimitiveComponent.CreateDynamicMaterialInstance` (`self.threat`) 0 null "None"))
  (`MaterialInstanceDynamic.SetScalarParameterValue` _returnvalue "Alpha" 0.0))

(fn `MarkAsPreMove`
  (`MaterialInstanceDynamic.SetScalarParameterValue` (`self.select_dynamic_material`) "Border Thickness" 0.85))

(fn `SetHoldedPiece`
  (params (piece :type "/Game/Blueprints/Pieces/Piece Object Reference"))
  (`/Engine/EditorBlueprintResources/StandardMacros.IsValid` piece
    (:`Is Valid`
      (bind _name (`/Game/Blueprints/Pieces/Piece.GetPieceName` piece))
      (set `self.holded_piece_info` (make `/Game/Blueprints/Structs/PieceInfo` _name (`/Game/Blueprints/Pieces/Piece.is_black` piece)))
      (set `self.holded_piece` piece))
    (:`Is Not Valid`
      (set `self.holded_piece_info` (make `/Game/Blueprints/Structs/PieceInfo` "NewEnumerator6")))))

(fn `SetHoldedPieceInfo`
  (params (piece :type "/Game/Blueprints/Pieces/Piece Object Reference"))
  (`/Engine/EditorBlueprintResources/StandardMacros.IsValid` piece
    (:`Is Valid`
      (bind _name (`/Game/Blueprints/Pieces/Piece.GetPieceName` piece))
      (set `self.holded_piece_info` (make `/Game/Blueprints/Structs/PieceInfo` _name (`/Game/Blueprints/Pieces/Piece.is_black` piece))))
    (:`Is Not Valid`
      (set `self.holded_piece_info` (make `/Game/Blueprints/Structs/PieceInfo` "NewEnumerator6")))))

(fn `UnMarkAsPreMove`
  (`MaterialInstanceDynamic.SetScalarParameterValue` (`self.select_dynamic_material`) "Border Thickness" 1.0))

(fn `UserConstructionScript`)