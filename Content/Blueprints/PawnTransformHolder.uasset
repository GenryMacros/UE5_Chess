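; PawnTransformHolder displays piece options, apparently for chess pawn promotion, as spheres fanned in a vertical arc around its location.
; SpawnSpheres spawns one PieceSphere per slot at a shared origin, assigns its piece type and color, and precomputes its raised arc position.
; A Timeline then lerps each sphere from its current location toward that target.
; Destroy removes all spheres along with the holder.
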(event `SpawnSpheres`
  (params (is_black :type Boolean))
  (`self.Spawn spheres` is_black)
  (bind (_direction _alpha) (`Timeline|Timeline` :!via `PlayFromStart`)
    (:`Update`
      (for (_ _array_index) (`self.spheres`)
        (bind _output (`|GetArrayItem` (`self.spheres`) _array_index))
        (`self.K2_SetActorLocation` _output (`KismetMathLibrary.VLerp` (`self.K2_GetActorLocation` _output) (`|GetArrayItem` (`self.spheres_final`) _array_index) _alpha) false false)))))

(fn `Destroy`
  (for _array_element (`self.spheres`)
    (`/Engine/EditorBlueprintResources/StandardMacros.IsValid` _array_element
      (:`Is Valid`
        (`self.K2_DestroyActor` _array_element))))
  (`self.K2_DestroyActor`))

(fn `Spawn spheres`
  (params (is_black :type Boolean))
  (locals (spheres_count :type Integer :default 4) (radius :type "Float (double-precision)" :default 210.0))
  (bind _spheres_count (`local.spheres_count`))
  (bind _returnvalue (+ (`self.K2_GetActorLocation`) (`KismetMathLibrary.MakeVector` -50.0 -52.0)))
  (for _index (range 1 (+ _spheres_count 1))
    (`KismetArrayLibrary.Array_Add` (`self.spheres_final`) (+ (+ (* (`KismetMathLibrary.GetForwardVector` (`KismetMathLibrary.MakeRotator` 0.0 (`KismetMathLibrary.Conv_IntToDouble` (* _index (/ 150 _spheres_count))) 90.0)) (`local.radius`)) (`KismetMathLibrary.MakeVector` 0.0 0.0 100.0)) _returnvalue))
    (bind _returnvalue_2 (`|SpawnActorFromClass` "/Game/Blueprints/PieceSphere.PieceSphere_C" (`KismetMathLibrary.MakeTransform` _returnvalue) "Undefined" "OverrideRootScale" null null))
    (`/Game/Blueprints/PieceSphere.ML_SetPiece` _returnvalue_2 (`|GetArrayItem` (`self.pieces2spawn`) (- _index 1)) is_black)
    (`KismetArrayLibrary.Array_Add` (`self.spheres`) _returnvalue_2)))

(fn `UserConstructionScript`)