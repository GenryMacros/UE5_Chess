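; Game mode for two-player chess that starts the match, assigns colours and detects when the game is over.
; It tracks logged-in controllers, alternates colours from a random first pick, and on start spawns a MousePawn for each at the colour-tagged PlayerStart.
; Game-over detection temporarily applies each move of the side to move on ChessGameState and checks whether its king stays attacked, so IsCheckmate alone only tests for check.
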(event `self.ReceiveBeginPlay`
  (set `self.ready_controllers` 0)
  (bind _aschess_game_state (cast `/Game/Blueprints/Global/ChessGameState` (`GameplayStatics.GetGameState`)))
  (bind _output_get (set `self.game_state` _aschess_game_state))
  (set `self.next_player_color` (`KismetMathLibrary.RandomBool`))
  (`/Game/Blueprints/Global/ChessGameState.ML_Load` _output_get))

(event `SV_RequestPlayerData`
  (params (player :type "/Game/Blueprints/Global/ChessPlayerController Object Reference"))
  (bind _output_get (set `/Game/Blueprints/Global/ChessPlayerController.is_black` (`self.next_player_color`) player))
  (set `self.next_player_color` (not _output_get)))

(event `SV_StartGame`
  (for _array_element (`self.player_controllers`)
    (`self.Spawn` _array_element))
  (cast `/Game/Blueprints/Global/ChessGameState` (`GameplayStatics.GetGameState`)))

(event `self.K2_PostLogin`
  (params (NewPlayer :type "PlayerController Object Reference"))
  (bind _player_controllers (`self.player_controllers`))
  (bind _aschess_player_controller (cast `/Game/Blueprints/Global/ChessPlayerController` NewPlayer))
  (`KismetArrayLibrary.Array_Add` _player_controllers _aschess_player_controller)
  (if (== 2 (`KismetArrayLibrary.Array_Length` _player_controllers))
    (`self.SV_StartGame`)))

(event `self.K2_OnLogout`
  (params (ExitingController :type "Controller Object Reference"))
  (bind _aschess_player_controller (cast `/Game/Blueprints/Global/ChessPlayerController` ExitingController))
  (`KismetArrayLibrary.Array_RemoveItem` (`self.player_controllers`) _aschess_player_controller)
  (`/Engine/EditorBlueprintResources/StandardMacros.DecrementInt` (`self.ready_controllers`)))

(fn `AssignColors`
  (bind _returnvalue (`KismetMathLibrary.RandomBool`))
  (bind _player_controllers (`self.player_controllers`))
  (set `/Game/Blueprints/Global/ChessPlayerController.is_black` _returnvalue (`|GetArrayItem` _player_controllers))
  (set `/Game/Blueprints/Global/ChessPlayerController.is_black` (not _returnvalue) (`|GetArrayItem` _player_controllers 1)))

(fn `AssignControlledPieces`
  (for _ (`/Game/Blueprints/Global/ChessGameState.pieces` (`self.game_state`))
    (for _ (`self.player_controllers`)
      _)))

(fn `CheckIfGameOver`
  (returns (is_gg :type Boolean))
  (locals (piece_original_tile :type "/Game/Blueprints/Tile Object Reference"))
  (for _array_element (`/Game/Blueprints/Global/ChessGameState.pieces` (`self.game_state`))
    (set `local.piece_original_tile` (`/Game/Blueprints/Pieces/Piece.tile` _array_element))
    (if (== (`/Game/Blueprints/Global/ChessGameState.is_black_turn` (`self.game_state`)) (`/Game/Blueprints/Pieces/Piece.is_black` _array_element))
      (bind _tiles (`/Game/Blueprints/Global/ChessGameState.GetTilesAttackedByPiece` (`self.game_state`) _array_element))
      (for _array_element_2 _tiles
        (if (!= _array_element_2 (`local.piece_original_tile`))
          (set `/Game/Blueprints/Pieces/Piece.tile` _array_element_2 _array_element)
          (`/Game/Blueprints/Tile.SetHoldedPieceInfo` (`local.piece_original_tile`) null)
          (`/Game/Blueprints/Tile.SetHoldedPieceInfo` _array_element_2 _array_element)
          (bind _tiles_under_attack (`/Game/Blueprints/Global/ChessGameState.GetAllAttackedTiles` (`self.game_state`) (not (`/Game/Blueprints/Global/ChessGameState.is_black_turn` (`self.game_state`)))))
          (bind _is_checkmate (`self.IsCheckmate` _tiles_under_attack))
          (set `/Game/Blueprints/Pieces/Piece.tile` (`local.piece_original_tile`) _array_element)
          (`/Game/Blueprints/Tile.SetHoldedPieceInfo` (`local.piece_original_tile`) _array_element)
          (`/Game/Blueprints/Tile.SetHoldedPieceInfo` _array_element_2 (`/Game/Blueprints/Tile.holded_piece` _array_element_2))
          (if (not _is_checkmate)
            (return false))))))
  (return true))

(fn `Get Spawn Transform`
  (params (is_black :type Boolean))
  (returns (transform :type "Transform Structure"))
  (locals (searched_tag :type String))
  (if is_black
    (set `local.searched_tag` "black")
    (else
      (set `local.searched_tag` "white")))
  (bind _outactors (`GameplayStatics.GetAllActorsOfClass` "/Script/Engine.PlayerStart"))
  (for _array_element _outactors
    (if (== (`local.searched_tag`) (`KismetStringLibrary.Conv_NameToString` (`PlayerStart.PlayerStartTag` _array_element)))
      (return (`self.GetTransform` _array_element)))))

(fn `IsCheckmate`
  (params (attacked_tiles :type "Array of /Game/Blueprints/Tile Object Reference"))
  (returns (is_checkmate :type Boolean))
  (locals (checking_king :type "/Game/Blueprints/Pieces/Piece Object Reference"))
  (bind _game_state (`self.game_state`))
  (if (`/Game/Blueprints/Global/ChessGameState.is_black_turn` (`self.game_state`))
    (bind _output_get (set `local.checking_king` (`/Game/Blueprints/Global/ChessGameState.black_king` _game_state)))
    (return (!= (`KismetArrayLibrary.Array_Find` attacked_tiles (`/Game/Blueprints/Pieces/Piece.tile` _output_get)) -1))
    (else
      (bind _output_get_2 (set `local.checking_king` (`/Game/Blueprints/Global/ChessGameState.white_king` _game_state)))
      (return (!= (`KismetArrayLibrary.Array_Find` attacked_tiles (`/Game/Blueprints/Pieces/Piece.tile` _output_get_2)) -1)))))

(fn `IsReady2Start`
  (returns (is_ready :type Boolean))
  (return (== 2 (`KismetArrayLibrary.Array_Length` (`self.player_controllers`)))))

(fn `PostGameOver`
  (`/Game/Blueprints/Global/ChessGameState.Move2GameOverState` (`self.game_state`)))

(fn `RequestColor`
  (returns (is_black :type Boolean))
  (locals (ret :type Boolean))
  (bind _next_player_color (`self.next_player_color`))
  (set `local.ret` _next_player_color)
  (set `self.next_player_color` (not _next_player_color))
  (return (`local.ret`)))

(fn `Spawn`
  (params (player :type "/Game/Blueprints/Global/ChessPlayerController Object Reference"))
  (bind _returnvalue (`Controller.K2_GetPawn` player))
  (`/Engine/EditorBlueprintResources/StandardMacros.IsValid` _returnvalue
    (:`Is Valid`
      (`self.K2_DestroyActor` _returnvalue))
    (:`Is Not Valid`
      _))
  (bind _transform (`self.Get Spawn Transform` (`/Game/Blueprints/Global/ChessPlayerController.is_black` player)))
  (bind _returnvalue_2 (`|SpawnActorFromClass` "/Game/Blueprints/MousePawn.MousePawn_C" (`KismetMathLibrary.MakeTransform` (`KismetMathLibrary.MakeVector` (.x (.location _transform)) (.y (.location _transform))) (.rotation _transform)) "Undefined" "OverrideRootScale" null null))
  (`Controller.Possess` player _returnvalue_2))

(fn `UserConstructionScript`)