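; Player controller for a multiplayer chess game, relaying player actions to the game state and answering turn, game-over and restart queries.
; BeginPlay requests player data from the game mode, reskins pieces and enables mouse events.
; SV_, CL_ and ML_ events route moves, resets and restart status between server and clients.
; For pawn promotion, it spawns a transform holder with selectable spheres, then passes the chosen sphere to ChessGameState.
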(event `self.ReceiveBeginPlay`
  (if true
    (bind _aschess_game_mode (cast `/Game/Blueprints/Global/ChessGameMode` (`GameplayStatics.GetGameMode`)))
    (`/Game/Blueprints/Global/ChessGameMode.SV_RequestPlayerData` _aschess_game_mode self)
    (bind _aschess_game_state (cast `/Game/Blueprints/Global/ChessGameState` (`GameplayStatics.GetGameState`)))
    (`/Game/Blueprints/Global/ChessGameState.ReskinPieces` _aschess_game_state)
    (set `self.game_state` _aschess_game_state)
    (set `self.bEnableMouseOverEvents` true)
    (set `self.bEnableClickEvents` true)))

(event `SV_EV_ChangeActorLocation`
  (params (actor :type "Actor Object Reference") (destination :type "Vector Structure"))
  (`self.K2_SetActorLocation` actor destination false false))

(event `SV_EV_MakeMove`
  (params (piece :type "/Game/Blueprints/Pieces/Piece Object Reference") (new_tile :type "/Game/Blueprints/Tile Object Reference"))
  (bind _aschess_game_state (cast `/Game/Blueprints/Global/ChessGameState` (`GameplayStatics.GetGameState`)))
  (`/Game/Blueprints/Global/ChessGameState.MakeMove` _aschess_game_state piece new_tile self))

(event `SV_Switch2PawnTransformMode`
  (params (pawn :type "/Game/Blueprints/Pieces/Pawn Object Reference (by ref)"))
  (`/Engine/EditorBlueprintResources/StandardMacros.IsValid` pawn
    (:`Is Valid`
      (bind _returnvalue (`|SpawnActorFromClass` "/Game/Blueprints/PawnTransformHolder.PawnTransformHolder_C" (`KismetMathLibrary.MakeTransform` (+ (`self.K2_GetActorLocation` (`/Game/Blueprints/Pieces/Piece.tile` pawn)) (`KismetMathLibrary.MakeVector` 30.0 60.0))) "Undefined" "OverrideRootScale" null null))
      (bind _output_get (set `/Game/Blueprints/Pieces/Pawn.transformer` _returnvalue pawn))
      (`/Game/Blueprints/PawnTransformHolder.SpawnSpheres` _output_get (`/Game/Blueprints/Pieces/Piece.is_black` pawn))
      (set `self.is_pawn_transform_mode` true))))

(event `SV_ToRestartState`
  (`/Game/Blueprints/Global/ChessGameState.2RestartMode` (`self.game_state`)))

(event `SV_FinalizePawnTransformation`
  (params (selected_piece_sphere :type "/Game/Blueprints/PieceSphere Object Reference"))
  (bind _aschess_game_state (cast `/Game/Blueprints/Global/ChessGameState` (`GameplayStatics.GetGameState`)))
  (`/Game/Blueprints/Global/ChessGameState.FinalizePawnTransformation` _aschess_game_state null selected_piece_sphere)
  (set `self.is_pawn_transform_mode` false))

(event `CL_RestartWait`
  (`/Game/Blueprints/UI/UIController.SetRestartWait` (`/Game/Blueprints/Global/ChessGameState.ui_controller` (`self.game_state`))))

(event `SV_ResetGame`
  (`/Game/Blueprints/Global/ChessGameState.SV_Reset` (`self.game_state`)))

(event `SV_DeclineReset`
  (`/Game/Blueprints/Global/ChessGameState.ML_DeclineReset` (`self.game_state`)))

(event `ML_MakeNonInitiator`
  (set `self.is_restart initiator` false))

(fn `Is In Restart`
  (returns (is_restart :type Boolean))
  (bind _game_state (`self.game_state`))
  (`/Engine/EditorBlueprintResources/StandardMacros.IsValid` _game_state
    (:`Is Valid`
      (return (`/Game/Blueprints/Global/ChessGameState.is_restart_state` _game_state)))
    (:`Is Not Valid`
      (bind _aschess_game_state (cast `/Game/Blueprints/Global/ChessGameState` (`GameplayStatics.GetGameState`)))
      (return (`/Game/Blueprints/Global/ChessGameState.is_restart_state` _aschess_game_state)))))

(fn `IsGGState`
  (returns (is_gg :type Boolean))
  (bind _game_state (`self.game_state`))
  (`/Engine/EditorBlueprintResources/StandardMacros.IsValid` _game_state
    (:`Is Valid`
      _)
    (:`Is Not Valid`
      (bind _aschess_game_state (cast `/Game/Blueprints/Global/ChessGameState` (`GameplayStatics.GetGameState`)))
      (set `self.game_state` _aschess_game_state)))
  (return (`/Game/Blueprints/Global/ChessGameState.is_game_over_state` _game_state)))

(fn `IsMyTurn`
  (returns (is_my_turn :type Boolean))
  (bind _aschess_game_state (cast `/Game/Blueprints/Global/ChessGameState` (`GameplayStatics.GetGameState`)))
  (return (== (`self.is_black`) (`/Game/Blueprints/Global/ChessGameState.is_black_turn` _aschess_game_state))))

(fn `Make Move`
  (params (Piece :type "Actor Object Reference"))
  (`/Engine/EditorBlueprintResources/StandardMacros.IsValid` null))

(fn `UserConstructionScript`)