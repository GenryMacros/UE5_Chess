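; Networked chess game state that owns the pieces, turn, material score, check and game-over flags.
; It spawns pieces from the JSON-loaded TileMap and handles moves, captures to a Graveyard, pawn promotion and board resets.
; IsMovePossible simulates tile swaps to reject moves leaving the king attacked, and MoveAnimator moves the pieces.
; After each move it passes the turn, rescores and asks ChessGameMode about check and game over, while RepNotifies update skins and restart UI.
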(event `self.ReceiveBeginPlay`
  (bind _returnvalue (`KismetMathLibrary.MakeTransform` (0.0 0.0 0.0)))
  (bind _returnvalue_2 (`|SpawnActorFromClass` "/Game/Blueprints/Graveyard.Graveyard_C" _returnvalue "Undefined" "OverrideRootScale" null null))
  (set `self.graveyard` _returnvalue_2)
  (bind _returnvalue_3 (`|SpawnActorFromClass` "/Game/Blueprints/PiecesMoveAnimator.PiecesMoveAnimator_C" _returnvalue "Undefined" "OverrideRootScale" null null))
  (set `self.move_animator` _returnvalue_3)
  (bind _outactors (`GameplayStatics.GetAllActorsOfClass` "/Game/Blueprints/UI/UIController.UIController_C"))
  (set `self.ui_controller` (`|GetArrayItem` _outactors)))

(event `ML_Load`
  (set `self.white_material` "/Game/EF_FirstFloor/Common/Materials/Wood/OLD/wood_a_Mat_Inst.wood_a_Mat_Inst")
  (set `self.black_material` "/Game/EF_FirstFloor/Common/Materials/Wood/WM_WoodRough_a_mat.WM_WoodRough_a_mat")
  (bind _outactors (`GameplayStatics.GetAllActorsOfClass` "/Game/Blueprints/TileMap.TileMap_C"))
  (set `self.tile_map` (`|GetArrayItem` _outactors))
  (`/Game/Blueprints/TileMap.ExportFromJson` (`self.tile_map`))
  (`self.SpawnPieces`))

(event `MakeMove`
  (params (Piece :type "/Game/Blueprints/Pieces/Piece Object Reference (by ref)") (NewTile :type "/Game/Blueprints/Tile Object Reference (by ref)") (player :type "/Game/Blueprints/Global/ChessPlayerController Object Reference (by ref)"))
  (bind _tile_map (`self.tile_map`))
  (bind _new_tile_temp (`self.new_tile_temp`))
  (bind _holded_piece (`/Game/Blueprints/Tile.holded_piece` _new_tile_temp))
  (`/Engine/EditorBlueprintResources/StandardMacros.IsValid` Piece
    (:`Is Valid`
      (`/Engine/EditorBlueprintResources/StandardMacros.IsValid` NewTile
        (:`Is Valid`
          (bind _is_possible (`self.IsMovePossible` Piece NewTile))
          (if _is_possible
            (set `self.new_tile_temp` NewTile)
            (else
              (set `self.new_tile_temp` (`/Game/Blueprints/Pieces/Piece.tile` Piece))))
          (`/Engine/EditorBlueprintResources/StandardMacros.IsValid` _holded_piece
            (:`Is Valid`
              (if (not (== (`/Game/Blueprints/Pieces/Piece.tile` Piece) _new_tile_temp))
                (`/Game/Blueprints/Graveyard.Bury` (`self.graveyard`) _holded_piece (`self.move_animator`))
                (`self.RemovePieceFromGame` _holded_piece)))
            (:`Is Not Valid`
              _))
          (bind _location (`self.CorrectDestinationVector` (`self.K2_GetActorLocation` _new_tile_temp) Piece))
          (`/Game/Blueprints/PiecesMoveAnimator.MovePieceTo` (`self.move_animator`) Piece _location)
          (bind _is_belongs (`/Game/Blueprints/Tile.IsPieceBelongs2Tile` _new_tile_temp Piece))
          (if (not _is_belongs)
            (`/Game/Blueprints/TileMap.ML_Make Non Threat All` _tile_map (not (`self.is_black_turn`)))
            (bind (_is_moved _piece _to) (`/Game/Blueprints/Pieces/Piece.PostMove` Piece _new_tile_temp _tile_map))
            (`/Game/Blueprints/TileMap.SwapTiles` (`self.tile_map`) (`/Game/Blueprints/Pieces/Piece.tile` Piece) _new_tile_temp)
            (if _is_moved
              (cast `/Game/Blueprints/Pieces/King` Piece
                (:`then`
                  (`/Game/Blueprints/PiecesMoveAnimator.MovePieceTo` (`self.move_animator`) _piece _to)
                  (`self.PostMoveJob` :!label _label))
                (:`CastFailed`
                  (bind _aspawn (cast `/Game/Blueprints/Pieces/Pawn` Piece))
                  (`/Game/Blueprints/Global/ChessPlayerController.SV_Switch2PawnTransformMode` player _aspawn)
                  (set `self.transforming_pawn` _aspawn)))
              (else
                (goto _label)))))))))

(event `FinalizePawnTransformation`
  (params (pawn :type "/Game/Blueprints/Pieces/Pawn Object Reference") (selected_sphere :type "/Game/Blueprints/PieceSphere Object Reference"))
  (`self.CompletePawnTransformation` selected_sphere (`self.transforming_pawn`))
  (`self.PostMoveJob`))

(event `ML_DestroyTransformedPawn`
  (bind _transforming_pawn (`self.transforming_pawn`))
  (bind _outactors (`GameplayStatics.GetAllActorsOfClass` "/Game/Blueprints/PawnTransformHolder.PawnTransformHolder_C"))
  (for _array_element _outactors
    (`/Game/Blueprints/PawnTransformHolder.Destroy` _array_element))
  (`/Engine/EditorBlueprintResources/StandardMacros.IsValid` _transforming_pawn
    (:`Is Valid`
      (`self.K2_DestroyActor` _transforming_pawn))))

(event `self.ReceiveEndPlay`
  (params (EndPlayReason :type "EEndPlayReason Enum" :default "Destroyed"))
  (`self.K2_DestroyActor` (`self.graveyard`))
  (`self.K2_DestroyActor` (`self.move_animator`)))

(event `SV_MarkCheckMaker`
  (bind _king (`self.GetActiveKing`))
  (for _array_element (`self.pieces`)
    (if (== (not (`self.is_black_turn`)) (`/Game/Blueprints/Pieces/Piece.is_black` _array_element))
      (bind _selected_tiles (`/Game/Blueprints/Pieces/Piece.select` _array_element (`self.tile_map`)))
      (if (!= (`KismetArrayLibrary.Array_Find` _selected_tiles (`/Game/Blueprints/Pieces/Piece.tile` _king)) -1)
        (`self.ML_MakeThreat` (`/Game/Blueprints/Pieces/Piece.tile` _array_element))))))

(event `ML_MakeThreat`
  (params (tile :type "/Game/Blueprints/Tile Object Reference"))
  (`/Game/Blueprints/Tile.MakeThreat` tile))

(event `ML_Switch Player 2Pawn Transform Mode`
  (params (player :type "/Game/Blueprints/Global/ChessPlayerController Object Reference (by ref)") (pawn :type "/Game/Blueprints/Pieces/Pawn Object Reference (by ref)"))
  (`/Engine/EditorBlueprintResources/StandardMacros.IsValid` player
    (:`Is Valid`
      (`/Engine/EditorBlueprintResources/StandardMacros.IsValid` pawn
        (:`Is Valid`
          (bind _returnvalue (`|SpawnActorFromClass` "/Game/Blueprints/PawnTransformHolder.PawnTransformHolder_C" (`KismetMathLibrary.MakeTransform` (+ (`self.K2_GetActorLocation` (`/Game/Blueprints/Pieces/Piece.tile` pawn)) (`KismetMathLibrary.MakeVector` 30.0 60.0))) "Undefined" "OverrideRootScale" null null))
          (bind _output_get (set `/Game/Blueprints/Pieces/Pawn.transformer` _returnvalue pawn))
          (`/Game/Blueprints/PawnTransformHolder.SpawnSpheres` _output_get (`/Game/Blueprints/Pieces/Piece.is_black` pawn))
          (`/Game/Blueprints/Global/ChessPlayerController.SV_Switch2PawnTransformMode` player pawn))))))

(event `Move2GameOverState`
  (`/Game/Blueprints/UI/UIController.SetGameOver` (`self.ui_controller`) (not (`self.is_black_turn`)))
  (set `self.is_game_over_state` true))

(event `2RestartMode`
  (set `self.is_restart_state` true))

(event `ML_DeclineReset`
  (set `self.is_restart_state` false)
  (bind _aschess_game_mode (cast `/Game/Blueprints/Global/ChessGameMode` (`GameplayStatics.GetGameMode`)))
  (for _array_element (`/Game/Blueprints/Global/ChessGameMode.player_controllers` _aschess_game_mode)
    (`/Game/Blueprints/Global/ChessPlayerController.ML_MakeNonInitiator` _array_element)))

(event `SV_Reset`
  (for _array_element (`self.pieces`)
    (bind _tile (`/Game/Blueprints/Pieces/Piece.tile` _array_element))
    (set `/Game/Blueprints/Tile.holded_piece` null _tile)
    (set `/Game/Blueprints/Tile.holded_piece_info` (struct) _tile)
    (bind _original_tile (`/Game/Blueprints/Pieces/Piece.original_tile` _array_element))
    (`/Game/Blueprints/Tile.SetHoldedPiece` _original_tile _array_element)
    (set `/Game/Blueprints/Pieces/Piece.tile` _original_tile _array_element)
    (bind _location (`self.CorrectDestinationVector` (`self.K2_GetActorLocation` _original_tile) _array_element))
    (`/Game/Blueprints/PiecesMoveAnimator.FastMovePieceTo` (`self.move_animator`) _array_element _location))
  (for _array_element_2 (`/Game/Blueprints/Graveyard.bodies` (`self.graveyard`))
    (`KismetArrayLibrary.Array_Add` (`self.pieces`) _array_element_2)
    (bind _original_tile_2 (`/Game/Blueprints/Pieces/Piece.original_tile` _array_element_2))
    (`/Game/Blueprints/Tile.SetHoldedPiece` _original_tile_2 _array_element_2)
    (set `/Game/Blueprints/Pieces/Piece.tile` _original_tile_2 _array_element_2)
    (bind _location_2 (`self.CorrectDestinationVector` (`self.K2_GetActorLocation` _original_tile_2) _array_element_2))
    (`/Game/Blueprints/PiecesMoveAnimator.FastMoveResizePieceTo` (`self.move_animator`) _array_element_2 _location_2 (* (`self.GetActorScale3D` _array_element_2) (2.0 2.0 2.0))))
  (`/Game/Blueprints/Graveyard.ClearBodies` (`self.graveyard`))
  (set `self.is_game_over_state` false)
  (set `self.is_game_over_state` false)
  (set `self.is_checkmate` false)
  (set `self.is_black_turn` false)
  (set `self.is_restart_state` false)
  (bind _aschess_game_mode (cast `/Game/Blueprints/Global/ChessGameMode` (`GameplayStatics.GetGameMode`)))
  (for _array_element_3 (`/Game/Blueprints/Global/ChessGameMode.player_controllers` _aschess_game_mode)
    (`/Game/Blueprints/Global/ChessPlayerController.ML_MakeNonInitiator` _array_element_3)))

(fn `CompletePawnTransformation`
  (params (selected_sphere :type "/Game/Blueprints/PieceSphere Object Reference") (pawn :type "/Game/Blueprints/Pieces/Pawn Object Reference"))
  (bind _tile (`/Game/Blueprints/Pieces/Piece.tile` pawn))
  (bind _pieces (`self.pieces`))
  (set `/Game/Blueprints/Tile.holded_piece_info` (make `/Game/Blueprints/Structs/PieceInfo` (`/Game/Blueprints/PieceSphere.repr_piece` selected_sphere) (`/Game/Blueprints/Pieces/Piece.is_black` pawn)) _tile)
  (bind _piece (`self.SpawnSignlePiece` _tile))
  (`KismetArrayLibrary.Array_RemoveItem` _pieces pawn)
  (`KismetArrayLibrary.Array_Add` _pieces _piece)
  (`self.ML_DestroyTransformedPawn`))

(fn `CorrectDestinationVector`
  (params (destination :type "Vector Structure") (moved_piece :type "/Game/Blueprints/Pieces/Piece Object Reference"))
  (returns (location :type "Vector Structure"))
  (locals (corrected_location :type "Vector Structure"))
  (cast `/Game/Blueprints/Pieces/Knight` moved_piece
    (:`then`
      (if (`/Game/Blueprints/Pieces/Piece.is_black` moved_piece)
        (set `local.corrected_location` (+ (`KismetMathLibrary.MakeVector` 52.0 -44.0 36.0) destination))
        (else
          (set `local.corrected_location` (+ destination (`KismetMathLibrary.MakeVector` -52.0 44.0 36.0))))))
    (:`CastFailed`
      (set `local.corrected_location` (+ destination (`KismetMathLibrary.MakeVector` -44.0 -52.0 36.0)))))
  (return (`local.corrected_location`)))

(fn `GetActiveKing`
  (returns (king :type "/Game/Blueprints/Pieces/King Object Reference"))
  (if (`self.is_black_turn`)
    (return (`self.black_king`))
    (else
      (return (`self.white_king`)))))

(fn `GetAllAttackedTiles`
  (params (is_black_attacks :type Boolean))
  (returns (tiles_under_attack :type "Array of /Game/Blueprints/Tile Object Reference"))
  (locals (attacked :type "Array of /Game/Blueprints/Tile Object Reference"))
  (for _array_element (`self.pieces`)
    (if (== is_black_attacks (`/Game/Blueprints/Pieces/Piece.is_black` _array_element))
      (bind _tiles (`self.GetTilesAttackedByPiece` _array_element))
      (for _array_element_2 _tiles
        (`KismetArrayLibrary.Array_Add` (`local.attacked`) _array_element_2))))
  (return (`local.attacked`)))

(fn `GetTileMap`
  (returns (tile_map :type "/Game/Blueprints/TileMap Object Reference"))
  (return (`self.tile_map`)))

(fn `GetTilesAttackedByPiece`
  (params (piece :type "/Game/Blueprints/Pieces/Piece Object Reference"))
  (returns (tiles :type "Array of /Game/Blueprints/Tile Object Reference"))
  (bind _selected_tiles (`/Game/Blueprints/Pieces/Piece.select` piece (`self.tile_map`)))
  (return _selected_tiles))

(fn `IsMovePossible`
  (params (piece :type "/Game/Blueprints/Pieces/Piece Object Reference") (destination :type "/Game/Blueprints/Tile Object Reference"))
  (returns (is_possible :type Boolean))
  (locals (piece_original_tile :type "/Game/Blueprints/Tile Object Reference") (remembered_piece :type "/Game/Blueprints/Pieces/Piece Object Reference") (remembered_piece_info :type "/Game/Blueprints/Structs/PieceInfo Structure"))
  (bind _remembered_piece (`local.remembered_piece`))
  (bind _holded_piece (`/Game/Blueprints/Tile.holded_piece` destination))
  (bind _output_get (set `local.piece_original_tile` (`/Game/Blueprints/Pieces/Piece.tile` piece)))
  (if (!= destination _output_get)
    (`/Engine/EditorBlueprintResources/StandardMacros.IsValid` _holded_piece
      (:`Is Valid`
        (set `local.remembered_piece` _holded_piece))
      (:`Is Not Valid`
        (set `local.remembered_piece` null)))
    (set `local.remembered_piece_info` (`/Game/Blueprints/Tile.holded_piece_info` destination))
    (`/Game/Blueprints/TileMap.SwapTiles` (`self.tile_map`) (`local.piece_original_tile`) destination)
    (bind _tiles_under_attack (`self.GetAllAttackedTiles` (not (`/Game/Blueprints/Pieces/Piece.is_black` piece))))
    (bind _aschess_game_mode (cast `/Game/Blueprints/Global/ChessGameMode` (`GameplayStatics.GetGameMode`)))
    (bind _is_checkmate (`/Game/Blueprints/Global/ChessGameMode.IsCheckmate` _aschess_game_mode _tiles_under_attack))
    (`/Game/Blueprints/TileMap.SwapTiles` (`self.tile_map`) destination (`local.piece_original_tile`))
    (set `/Game/Blueprints/Tile.holded_piece` _remembered_piece destination)
    (set `/Game/Blueprints/Tile.holded_piece_info` (`local.remembered_piece_info`) destination)
    (`/Engine/EditorBlueprintResources/StandardMacros.IsValid` _remembered_piece
      (:`Is Valid`
        (set `/Game/Blueprints/Pieces/Piece.tile` destination _remembered_piece))
      (:`Is Not Valid`
        _))
    (if _is_checkmate
      (return false)
      (else
        (return true)))
    (else
      (return true))))

(fn `MarkCheckMaker`
  (locals (targeted_king :type "/Game/Blueprints/Pieces/Piece Object Reference"))
  (if (`self.is_black_turn`)
    (set `local.targeted_king` (`self.black_king`))
    (else
      (set `local.targeted_king` (`self.white_king`))))
  (for _array_element (`self.pieces`)
    (if (== (not (`self.is_black_turn`)) (`/Game/Blueprints/Pieces/Piece.is_black` _array_element))
      (bind _selected_tiles (`/Game/Blueprints/Pieces/Piece.select` _array_element (`self.tile_map`)))
      (if (!= (`KismetArrayLibrary.Array_Find` _selected_tiles (`/Game/Blueprints/Pieces/Piece.tile` (`local.targeted_king`))) -1)
        (`/Game/Blueprints/Tile.MakeThreat` (`/Game/Blueprints/Pieces/Piece.tile` _array_element))))))

(fn `MarkKingAsCheckmated`
  (params (is_checkmate :type Boolean))
  (bind _white_king (`self.white_king`))
  (bind _black_king (`self.black_king`))
  (if is_checkmate
    (if (`self.is_black_turn`)
      (set `/Game/Blueprints/Pieces/King.is_in_checkmate` false _white_king)
      (set `/Game/Blueprints/Pieces/King.is_in_checkmate` true _black_king)
      (else
        (set `/Game/Blueprints/Pieces/King.is_in_checkmate` false _black_king)
        (set `/Game/Blueprints/Pieces/King.is_in_checkmate` true _white_king)))
    (else
      (set `/Game/Blueprints/Pieces/King.is_in_checkmate` false _white_king)
      (set `/Game/Blueprints/Pieces/King.is_in_checkmate` false _black_king))))

(fn `OnRep_is_restart_state`
  (if (`self.is_restart_state`)
    (bind _aschess_player_controller (cast `/Game/Blueprints/Global/ChessPlayerController` (`GameplayStatics.GetPlayerController` 0)))
    (if (not (`/Game/Blueprints/Global/ChessPlayerController.is_restart initiator` _aschess_player_controller))
      (`/Game/Blueprints/UI/UIController.SetRestart` (`self.ui_controller`)))
    (else
      (`/Game/Blueprints/UI/UIController.DestroyActiveWidget` (`self.ui_controller`)))))

(fn `OnRep_pieces`
  (if true
    (`self.ReskinPieces`)))

(fn `Pass Turn`
  (set `self.is_black_turn` (not (`self.is_black_turn`))))

(fn `PostMoveJob`
  (`self.Pass Turn`)
  (`self.RecalculateFieldValue`)
  (bind _aschess_game_mode (cast `/Game/Blueprints/Global/ChessGameMode` (`GameplayStatics.GetGameMode`)))
  (bind _tiles_under_attack (`self.GetAllAttackedTiles` (`self.is_black_turn`)))
  (bind _is_checkmate (`/Game/Blueprints/Global/ChessGameMode.IsCheckmate` _aschess_game_mode _tiles_under_attack))
  (bind _output_get (set `self.is_checkmate` _is_checkmate))
  (if _output_get
    (`self.MarkKingAsCheckmated` true)
    (`self.SV_MarkCheckMaker`)
    (bind _is_gg (`/Game/Blueprints/Global/ChessGameMode.CheckIfGameOver` _aschess_game_mode))
    (if _is_gg
      (`/Game/Blueprints/Global/ChessGameMode.PostGameOver` _aschess_game_mode))
    (else
      (`self.MarkKingAsCheckmated` false))))

(fn `PutPieceOnTile`
  (params (tile :type "/Game/Blueprints/Tile Object Reference") (piece :type "/Game/Blueprints/Pieces/Piece Object Reference") (is_black :type Boolean))
  (returns (ret_piece :type "/Game/Blueprints/Pieces/Piece Object Reference"))
  (bind _piece (`/Game/Blueprints/Pieces/Piece.CorrectLocation` piece is_black))
  (set `/Game/Blueprints/Tile.holded_piece` _piece tile)
  (set `/Game/Blueprints/Pieces/Piece.original_tile` tile _piece)
  (set `/Game/Blueprints/Pieces/Piece.tile` tile _piece)
  (bind _output_get (set `/Game/Blueprints/Pieces/Piece.is_black` is_black _piece))
  (if _output_get
    (`/Game/Blueprints/Pieces/Piece.Set Material` _piece (`self.black_material`))
    (else
      (`/Game/Blueprints/Pieces/Piece.Set Material` _piece (`self.white_material`))))
  (return _piece))

(fn `RecalculateFieldValue`
  (locals (score :type Integer) (mod :type Integer))
  (bind _score (`local.score`))
  (bind _mod (`local.mod`))
  (for _array_element (`/Game/Blueprints/TileMap.Tiles` (`self.tile_map`))
    (bind (_holded_piece_info_piece_name _holded_piece_info_is_black) (break `/Game/Blueprints/Structs/PieceInfo` (`/Game/Blueprints/Tile.holded_piece_info` _array_element)))
    (if _holded_piece_info_is_black
      (set `local.mod` -1)
      (else
        (set `local.mod` 1)))
    (switch `/Game/Blueprints/PieceNames` _holded_piece_info_piece_name
      (:`NewEnumerator0`
        (set `local.score` (+ _score (* 1 _mod))))
      (:`NewEnumerator1`
        (set `local.score` (+ _score (* 3 _mod))))
      (:`NewEnumerator2`
        (set `local.score` (+ _score (* 3 _mod))))
      (:`NewEnumerator3`
        (set `local.score` (+ _score (* 5 _mod))))
      (:`NewEnumerator4`
        (set `local.score` (+ _score (* 9 _mod))))))
  (set `self.field_value` (`KismetMathLibrary.Conv_IntToDouble` (`local.score`))))

(fn `RemoveAllPieces`
  (bind _pieces (`self.pieces`))
  (for _array_element _pieces
    (`/Engine/EditorBlueprintResources/StandardMacros.IsValid` _array_element
      (:`Is Valid`
        (`self.K2_DestroyActor` _array_element))))
  (`KismetArrayLibrary.Array_Clear` _pieces))

(fn `RemovePieceFromGame`
  (params (piece :type "/Game/Blueprints/Pieces/Piece Object Reference"))
  (bind _tile (`/Game/Blueprints/Pieces/Piece.tile` piece))
  (`KismetArrayLibrary.Array_RemoveItem` (`self.pieces`) piece)
  (set `/Game/Blueprints/Tile.holded_piece` null _tile)
  (set `/Game/Blueprints/Tile.holded_piece_info` (struct) _tile)
  (set `/Game/Blueprints/Pieces/Piece.tile` null piece))

(fn `ReskinPieces`
  (for _array_element (`self.pieces`)
    (`/Engine/EditorBlueprintResources/StandardMacros.IsValid` _array_element
      (:`Is Valid`
        (if (`/Game/Blueprints/Pieces/Piece.is_black` _array_element)
          (`/Game/Blueprints/Pieces/Piece.Set Material` _array_element (`self.black_material`))
          (else
            (`/Game/Blueprints/Pieces/Piece.Set Material` _array_element (`self.white_material`))))
        (`/Engine/EditorBlueprintResources/StandardMacros.IncrementInt` (`self.skins_set`))))))

(fn `SpawnPieces`
  (bind _tiles (`/Game/Blueprints/TileMap.Tiles` (`self.tile_map`)))
  (`self.RemoveAllPieces`)
  (for _index (range (`KismetArrayLibrary.Array_Length` _tiles))
    (bind _piece (`self.SpawnSignlePiece` (`|GetArrayItem` _tiles _index)))
    (`/Engine/EditorBlueprintResources/StandardMacros.IsValid` _piece
      (:`Is Valid`
        (`KismetArrayLibrary.Array_Add` (`self.pieces`) _piece)))))

(fn `SpawnSignlePiece`
  (params (tile :type "/Game/Blueprints/Tile Object Reference"))
  (returns (piece :type "/Game/Blueprints/Pieces/Piece Object Reference"))
  (locals (is_black :type Boolean) (tile_ref :type "/Game/Blueprints/Tile Object Reference"))
  (bind _coords_x (break `/Game/Blueprints/Structs/Coord` (`/Game/Blueprints/Tile.coords` (`local.tile_ref`))))
  (bind _output_get (set `local.tile_ref` tile))
  (bind (_holded_piece_info_piece_name _holded_piece_info_is_black) (break `/Game/Blueprints/Structs/PieceInfo` (`/Game/Blueprints/Tile.holded_piece_info` _output_get)))
  (set `local.is_black` _holded_piece_info_is_black)
  (switch `/Game/Blueprints/PieceNames` _holded_piece_info_piece_name
    (:`NewEnumerator0`
      (bind _returnvalue (`KismetMathLibrary.Conv_VectorToTransform` (`self.K2_GetActorLocation` _output_get)))
      (bind _returnvalue_2 (`|SpawnActorFromClass` "/Game/Blueprints/Pieces/Pawn.Pawn_C" _returnvalue "Undefined" "OverrideRootScale" null null))
      (set `/Game/Blueprints/Pieces/Pawn.initial_x` _coords_x _returnvalue_2)
      (bind _ret_piece (`self.PutPieceOnTile` (`local.tile_ref`) _returnvalue_2 (`local.is_black`)))
      (return _ret_piece))
    (:`NewEnumerator1`
      (bind _returnvalue_3 (`|SpawnActorFromClass` "/Game/Blueprints/Pieces/Bishop.Bishop_C" _returnvalue "Undefined" "OverrideRootScale" null null))
      (bind _ret_piece_2 (`self.PutPieceOnTile` (`local.tile_ref`) _returnvalue_3 (`local.is_black`)))
      (return _ret_piece_2))
    (:`NewEnumerator2`
      (bind _returnvalue_4 (`|SpawnActorFromClass` "/Game/Blueprints/Pieces/Knight.Knight_C" _returnvalue "Undefined" "OverrideRootScale" null null))
      (bind _ret_piece_3 (`self.PutPieceOnTile` (`local.tile_ref`) _returnvalue_4 (`local.is_black`)))
      (return _ret_piece_3))
    (:`NewEnumerator3`
      (bind _returnvalue_5 (`|SpawnActorFromClass` "/Game/Blueprints/Pieces/Rook.Rook_C" _returnvalue "Undefined" "OverrideRootScale" null null))
      (bind _ret_piece_4 (`self.PutPieceOnTile` (`local.tile_ref`) _returnvalue_5 (`local.is_black`)))
      (return _ret_piece_4))
    (:`NewEnumerator4`
      (bind _returnvalue_6 (`|SpawnActorFromClass` "/Game/Blueprints/Pieces/Queen.Queen_C" _returnvalue "Undefined" "OverrideRootScale" null null))
      (bind _ret_piece_5 (`self.PutPieceOnTile` (`local.tile_ref`) _returnvalue_6 (`local.is_black`)))
      (return _ret_piece_5))
    (:`NewEnumerator5`
      (bind _returnvalue_7 (`|SpawnActorFromClass` "/Game/Blueprints/Pieces/King.King_C" _returnvalue "Undefined" "OverrideRootScale" null null))
      (if (`local.is_black`)
        (set `self.black_king` _returnvalue_7)
        (else
          (set `self.white_king` _returnvalue_7)))
      (bind _ret_piece_6 (`self.PutPieceOnTile` (`local.tile_ref`) _returnvalue_7 (`local.is_black`)))
      (return _ret_piece_6))
    (:`NewEnumerator6`
      (return null))))

(fn `UserConstructionScript`)