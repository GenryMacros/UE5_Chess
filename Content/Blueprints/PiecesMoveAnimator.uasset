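; Actor that animates game pieces to new locations, optionally resizing them, in normal and fast variants.
; Timelines lerp from each piece's current transform toward the target every update.
; Both move events share one ready flag and queue, with queued moves replayed on the timeline that finishes.
; Fast move-resize has its own queue, while regular move-resize restarts its timeline immediately without queuing.
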(event `FastMovePieceTo`
  (params (piece :type "/Game/Blueprints/Pieces/Piece Object Reference") (destination :type "Vector Structure"))
  (bind _to_animate (`self.to_animate`))
  (bind (_current_payload_piece _current_payload_destionation) (break `/Game/Blueprints/Structs/AnimPayload` (`self.current_payload`)))
  (if (`self.is_ready`)
    (set `self.current_payload` (make `/Game/Blueprints/Structs/AnimPayload` piece destination))
    (bind (_direction _alpha) (`Timeline|Timeline_0` :!via `PlayFromStart` :!label _label)
      (:`Update`
        (set `self.is_ready` false)
        (bind (_returnvalue_x _returnvalue_y _returnvalue_z) (`KismetMathLibrary.BreakVector` (`KismetMathLibrary.VLerp` (`self.K2_GetActorLocation` _current_payload_piece) _current_payload_destionation _alpha)))
        (`self.K2_SetActorLocation` _current_payload_piece (`KismetMathLibrary.MakeVector` _returnvalue_x _returnvalue_y _returnvalue_z) false false))
      (:`Finished`
        (if (`KismetArrayLibrary.Array_IsEmpty` (`self.to_animate`))
          (set `self.is_ready` true)
          (else
            (set `self.current_payload` (`|GetArrayItem` _to_animate))
            (`KismetArrayLibrary.Array_Remove` _to_animate)
            (goto _label :!via `PlayFromStart`)))))
    (else
      (`KismetArrayLibrary.Array_Add` (`self.to_animate`) (make `/Game/Blueprints/Structs/AnimPayload` piece destination)))))

(event `MovePieceTo`
  (params (piece :type "/Game/Blueprints/Pieces/Piece Object Reference") (destination :type "Vector Structure"))
  (bind _to_animate (`self.to_animate`))
  (bind (_current_payload_piece _current_payload_destionation) (break `/Game/Blueprints/Structs/AnimPayload` (`self.current_payload`)))
  (if (`self.is_ready`)
    (set `self.current_payload` (make `/Game/Blueprints/Structs/AnimPayload` piece destination))
    (bind (_direction _alpha) (`Timeline|Timeline` :!via `PlayFromStart` :!label _label_2)
      (:`Update`
        (set `self.is_ready` false)
        (bind (_returnvalue_x _returnvalue_y _returnvalue_z) (`KismetMathLibrary.BreakVector` (`KismetMathLibrary.VLerp` (`self.K2_GetActorLocation` _current_payload_piece) _current_payload_destionation _alpha)))
        (`self.K2_SetActorLocation` _current_payload_piece (`KismetMathLibrary.MakeVector` _returnvalue_x _returnvalue_y _returnvalue_z) false false))
      (:`Finished`
        (if (`KismetArrayLibrary.Array_IsEmpty` (`self.to_animate`))
          (set `self.is_ready` true)
          (else
            (set `self.current_payload` (`|GetArrayItem` _to_animate))
            (`KismetArrayLibrary.Array_Remove` _to_animate)
            (goto _label_2 :!via `PlayFromStart`)))))
    (else
      (`KismetArrayLibrary.Array_Add` (`self.to_animate`) (make `/Game/Blueprints/Structs/AnimPayload` piece destination)))))

(event `MoveResizePieceTo`
  (params (Piece :type "/Game/Blueprints/Pieces/Piece Object Reference") (Destination :type "Vector Structure") (scale :type "Vector Structure"))
  (bind (_direction _location_alpha _scale_alpha) (`Timeline|ScaleMove_Timeline` :!via `PlayFromStart`)
    (:`Update`
      (`self.K2_SetActorLocation` Piece (`KismetMathLibrary.VLerp` (`self.K2_GetActorLocation` Piece) Destination _location_alpha) false false)
      (`self.SetActorScale3D` Piece (`KismetMathLibrary.VLerp` (`self.GetActorScale3D` Piece) scale _scale_alpha)))))

(event `FastMoveResizePieceTo`
  (params (Piece :type "/Game/Blueprints/Pieces/Piece Object Reference") (Destination :type "Vector Structure") (scale :type "Vector Structure"))
  (bind (_current_resize_payload_piece _current_resize_payload_destionation _current_resize_payload_final_scale) (break `/Game/Blueprints/Structs/AnimResizePayload` (`self.current_resize_payload`)))
  (if (`self.is_ready_res`)
    (set `self.current_resize_payload` (make `/Game/Blueprints/Structs/AnimResizePayload` Piece Destination scale))
    (bind (_direction _location_alpha _scale_alpha) (`Timeline|Timeline_1` :!via `PlayFromStart` :!label _label_3)
      (:`Update`
        (set `self.is_ready_res` false)
        (`self.K2_SetActorLocation` _current_resize_payload_piece (`KismetMathLibrary.VLerp` (`self.K2_GetActorLocation` _current_resize_payload_piece) _current_resize_payload_destionation _location_alpha) false false)
        (`self.SetActorScale3D` _current_resize_payload_piece (`KismetMathLibrary.VLerp` (`self.GetActorScale3D` _current_resize_payload_piece) _current_resize_payload_final_scale _scale_alpha)))
      (:`Finished`
        (if (`KismetArrayLibrary.Array_IsEmpty` (`self.current_resize_[ayload`))
          (set `self.is_ready_res` true)
          (else
            (set `self.current_resize_payload` (`|GetArrayItem` (`self.current_resize_[ayload`)))
            (`KismetArrayLibrary.Array_Remove` (`self.current_resize_[ayload`))
            (goto _label_3 :!via `PlayFromStart`)))))
    (else
      (`KismetArrayLibrary.Array_Add` (`self.current_resize_[ayload`) (make `/Game/Blueprints/Structs/AnimResizePayload` Piece Destination scale)))))

(fn `IsEqual`
  (params (val1 :type "Float (double-precision)") (val2 :type "Float (double-precision)"))
  (returns (is_equal :type Boolean))
  (locals (equality_range :type "Float (double-precision)" :default 0.2))
  (bind _equality_range (`local.equality_range`))
  (return (and (<= val2 (+ val1 _equality_range)) (>= val2 (- val1 _equality_range)))))

(fn `UserConstructionScript`)